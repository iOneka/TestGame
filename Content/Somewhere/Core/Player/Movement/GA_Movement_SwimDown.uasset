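; Gameplay ability that makes the survival character swim down while active.
; On activation it caches the avatar, then starts a tick task that lowers the capsule a fixed step each tick, without delta-time scaling.
; Each tick also adds negatively scaled movement input, using the capsule's world Z as the direction's Z.
; The SwimDown InputCompleted gameplay event ends the tick task and the ability.
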(event `self.K2_ActivateAbilityFromEvent`
  (params (EventData :type "GameplayEventData Structure (by ref)"))
  (bind _as_ch_survival_character (`self.As CH Survival Character`))
  (bind _capsulecomponent (`Character.CapsuleComponent` _as_ch_survival_character))
  (bind (_returnvalue_x _returnvalue_y _returnvalue_z) (`KismetMathLibrary.BreakVector` (`SceneComponent.K2_GetComponentLocation` _capsulecomponent)))
  (`|ExecutionSequence`
    (:`then_0`
      ;[0 0 0] References
      (bind _ascharacter (cast `Character` (`self.GetAvatarActorFromActorInfo`)))
      (bind _output_get (set `self.Avatar as Character` _ascharacter))
      (bind _asch_survival_character (cast `/Game/Somewhere/Core/Player/CH_SurvivalCharacter` _output_get))
      (set `self.As CH Survival Character` _asch_survival_character))
    (:`then_1`
      (bind _asynctaskproxy (`AbilityTask_Tick.Tick`)
        (:`then`
          (set `self.Tick Async Task` _asynctaskproxy)
          (`AbilityTask_WaitGameplayEvent.WaitGameplayEvent` (struct :`TagName` "GameplayAbility.Movement.SwimDown.InputCompleted") null
            (:`EventReceived`
              (`GameplayTask.EndTask` (`self.Tick Async Task`))
              (`self.K2_EndAbility`))))
        (:`OnTick`
          (`SceneComponent.K2_SetWorldLocation` _capsulecomponent (`KismetMathLibrary.MakeVector` _returnvalue_x _returnvalue_y (- _returnvalue_z 2.0)) false false)
          (`Pawn.AddMovementInput` _as_ch_survival_character (`KismetMathLibrary.MakeVector` 0.0 0.0 _returnvalue_z) -1.0 false))))))