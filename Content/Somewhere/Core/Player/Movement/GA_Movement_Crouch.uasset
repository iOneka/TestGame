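; Gameplay Ability that makes the avatar Character crouch until a crouch input-completed event arrives.
; Activation caches the avatar as a Character, calls Crouch, then waits for that gameplay event to end the ability.
; UnCrouch runs on ability end, and the activation check blocks crouching while the owner's CharacterMovementComponent reports falling.
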(event `self.K2_ActivateAbility`
  (`|ExecutionSequence`
    (:`then_0`
      ;[0 0 0] References
      (bind _ascharacter (cast `Character` (`self.GetAvatarActorFromActorInfo`)))
      (set `self.Avatar as Character` _ascharacter))
    (:`then_1`
      (`Character.Crouch` (`self.Avatar as Character`))
      (`AbilityTask_WaitGameplayEvent.WaitGameplayEvent` (struct :`TagName` "GameplayAbility.Movement.Crouch.InputCompleted") null
        (:`EventReceived`
          (`self.K2_EndAbility`))))))

(event `self.K2_OnEndAbility`
  (params (bWasCancelled :type Boolean))
  (`Character.UnCrouch` (`self.Avatar as Character`)))

(fn `K2_CanActivateAbility`
  (params (ActorInfo :type "GameplayAbilityActorInfo Structure") (Handle :type "GameplayAbilitySpecHandle Structure"))
  (returns (RelevantTags :type "GameplayTagContainer Structure") (ReturnValue :type Boolean))
  (return (struct) (not (`NavMovementComponent.IsFalling` (`Actor.GetComponentByClass` ActorInfo_OwnerActor "/Script/Engine.CharacterMovementComponent")))))