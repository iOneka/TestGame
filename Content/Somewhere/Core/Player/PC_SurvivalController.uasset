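; Survival player controller that handles proximity voice chat and developer debug shortcuts.
; Voice input toggles on mobile, or on desktop uses push-to-talk or toggle per console variable, driving Opus capture and the character's server-updated talking widget.
; Development builds add a debug input context for ability-system, collision and ragdoll tools, while F9 teleports the linked character to fixed coordinates.
; On BeginPlay, non-local controllers initialize the PoachContainer.
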(event `EnhancedInput|/Game/Somewhere/Core/Input/UIContext/IA_VoiceChat`
  (params (ActionValue :type Boolean) (ElapsedSeconds :type "Float (double-precision)") (TriggeredSeconds :type "Float (double-precision)") (InputAction :type "InputAction Object Reference" :default "/Game/Somewhere/Core/Input/UIContext/IA_VoiceChat.IA_VoiceChat"))
  ;[0 0 0] Use Microphone
  (:`Started`
    (switch `EPlatform` (`PlatformStatics.GetPlatform`)
      (:`Mobile`
        ;;[0 0 0] Toggle на мобилке
        (bind _isa (`/Engine/EditorBlueprintResources/StandardMacros.FlipFlop`)
          (:`A`
            _)
          (:`B`
            _))
        (`self.Toggle Voice Chat` _isa))
      (:`Desktop`
        (if (`ConsoleUtils.GetBoolCVar` "Game.MicrophonePushToTalk")
          ;;[0 0 0] PushToTalk On
          (`self.Toggle Voice Chat` true)
          (else
            ;;[0 0 0] Toggle на ПК
            (bind _isa_2 (`/Engine/EditorBlueprintResources/StandardMacros.FlipFlop`)
              (:`A`
                _)
              (:`B`
                _))
            (`self.Toggle Voice Chat` _isa_2))))))
  (:`Completed`
    (switch `EPlatform` (`PlatformStatics.GetPlatform`)
      (:`Desktop`
        (if (`ConsoleUtils.GetBoolCVar` "Game.MicrophonePushToTalk")
          ;;[0 0 0] PushToTalk Off
          (`self.Toggle Voice Chat` false))))))

(event `EnhancedInput|/Game/Somewhere/Core/Input/Debug/IA_Debug_5`
  (params (ActionValue :type Boolean) (ElapsedSeconds :type "Float (double-precision)") (TriggeredSeconds :type "Float (double-precision)") (InputAction :type "InputAction Object Reference" :default "/Game/Somewhere/Core/Input/Debug/IA_Debug_5.IA_Debug_5")))

(event `EnhancedInput|/Game/Somewhere/Core/Input/Debug/IA_Debug_0`
  (params (ActionValue :type Boolean) (ElapsedSeconds :type "Float (double-precision)") (TriggeredSeconds :type "Float (double-precision)") (InputAction :type "InputAction Object Reference" :default "/Game/Somewhere/Core/Input/Debug/IA_Debug_0.IA_Debug_0"))
  ;[0 0 0 1 24] NUMPAD 0 - Debug AbilitySytem
  (:`Started`
    (`|ExecutionSequence`
      (:`then_0`
        (`/Engine/EditorBlueprintResources/StandardMacros.DoOnce` false
          (:`Completed`
            (`KismetSystemLibrary.ExecuteConsoleCommand` "showdebug abilitysystem" self))))
      (:`then_1`
        (`KismetSystemLibrary.ExecuteConsoleCommand` "AbilitySystem.Debug.NextCategory" self)))))

(event `self.OnPlayerCharacterLinked`
  (params (SomewhereCharacter :type "SomewhereCharacter Object Reference"))
  (if (`self.IsLocalController`)
    (`|ExecutionSequence`)
    (else
      (`|ExecutionSequence`))))

(event `EnhancedInput|/Game/Somewhere/Core/Input/Debug/IA_Debug_6`
  (params (ActionValue :type Boolean) (ElapsedSeconds :type "Float (double-precision)") (TriggeredSeconds :type "Float (double-precision)") (InputAction :type "InputAction Object Reference" :default "/Game/Somewhere/Core/Input/Debug/IA_Debug_6.IA_Debug_6")))

(event `self.ReceiveBeginPlay`
  (`parent.ReceiveBeginPlay`)
  (if (`self.IsLocalController`)
    (`|ExecutionSequence`
      (:`then_2`
        ;[0 0 0] Весёлые кнопочки
        (if (`LowEntryExtendedStandardLibrary.DevelopmentBuild`)
          (`EnhancedInputSubsystemInterface.AddMappingContext` (pcsubsystem `EnhancedInputLocalPlayerSubsystem` self) "/Game/Somewhere/Core/Input/Debug/IMC_DebugContext.IMC_DebugContext" 0 (struct)))))
    (else
      (`|ExecutionSequence`
        (:`then_0`
          (`ItemContainer.Initialize` (`self.Poach Container`) 11))))))

(event `Key|F9`
  (params (Key :type "Key Structure"))
  ;[0 0 0] CTP
  (:`Pressed`
    (`self.Event CTP`)))

(event `Event CTP`
  (bind _returnvalue (`self.GetLinkedSomewhereCharacter`))
  ;[0 0 0] CTP
  (`/Engine/EditorBlueprintResources/StandardMacros.IsValid` _returnvalue
    (:`Is Valid`
      (`self.K2_SetActorLocation` _returnvalue (1000.0 -58000.0 13500.0) false true))))

(event `EnhancedInput|/Game/Somewhere/Core/Input/Debug/IA_Debug_1`
  (params (ActionValue :type Boolean) (ElapsedSeconds :type "Float (double-precision)") (TriggeredSeconds :type "Float (double-precision)") (InputAction :type "InputAction Object Reference" :default "/Game/Somewhere/Core/Input/Debug/IA_Debug_1.IA_Debug_1"))
  ;[0 0 0 1 24] NUMPAD 1 - Show Collisions
  (:`Started`
    (`KismetSystemLibrary.ExecuteConsoleCommand` "show collision" self)
    (`KismetSystemLibrary.ExecuteConsoleCommand` "show collisionPawn" self)))

(event `EnhancedInput|/Game/Somewhere/Core/Input/Debug/IA_Debug_7`
  (params (ActionValue :type Boolean) (ElapsedSeconds :type "Float (double-precision)") (TriggeredSeconds :type "Float (double-precision)") (InputAction :type "InputAction Object Reference" :default "/Game/Somewhere/Core/Input/Debug/IA_Debug_7.IA_Debug_7")))

(event `EnhancedInput|/Game/Somewhere/Core/Input/Debug/IA_Debug_2`
  (params (ActionValue :type Boolean) (ElapsedSeconds :type "Float (double-precision)") (TriggeredSeconds :type "Float (double-precision)") (InputAction :type "InputAction Object Reference" :default "/Game/Somewhere/Core/Input/Debug/IA_Debug_2.IA_Debug_2"))
  ;[0 0 0 1 24] NUMPAD 2 - Hide HUD
  (:`Started`
    (`/Engine/EditorBlueprintResources/StandardMacros.FlipFlop`)))

(event `self.OnPlayerControllerReady`
  (params (SomewherePlayerController :type "SomewherePlayerController Object Reference")))

(event `EnhancedInput|/Game/Somewhere/Core/Input/Debug/IA_Debug_3`
  (params (ActionValue :type Boolean) (ElapsedSeconds :type "Float (double-precision)") (TriggeredSeconds :type "Float (double-precision)") (InputAction :type "InputAction Object Reference" :default "/Game/Somewhere/Core/Input/Debug/IA_Debug_3.IA_Debug_3"))
  ;[0 0 0 1 24] NUMPAD 3 - Ragdoll
  (:`Started`
    (bind _asch_survival_character (cast `/Game/Somewhere/Core/Player/CH_SurvivalCharacter` (`self.K2_GetPawn`)))
    (bind _isa (`/Engine/EditorBlueprintResources/StandardMacros.FlipFlop`)
      (:`A`
        _)
      (:`B`
        _))
    (`/Game/Somewhere/Core/Player/CH_SurvivalCharacter.Ragdoll` _asch_survival_character _isa)))

(event `EnhancedInput|/Game/Somewhere/Core/Input/Debug/IA_Debug_4`
  (params (ActionValue :type Boolean) (ElapsedSeconds :type "Float (double-precision)") (TriggeredSeconds :type "Float (double-precision)") (InputAction :type "InputAction Object Reference" :default "/Game/Somewhere/Core/Input/Debug/IA_Debug_4.IA_Debug_4")))

(fn `ctp`
  (`self.Event CTP`))

(fn `Toggle Voice Chat`
  (params (Toggle :type Boolean))
  (if Toggle
    (bind _returnvalue (`UniversalVoiceChat.VoiceChatWasInitAudioVoiceChatQuality`))
    (if (not _returnvalue)
      (`UniversalVoiceChat.VoiceChatInitAudioVoiceChatQuality` 48000))
    (`UniversalVoiceChat.VoiceChatStartSpeak` false true 0 true 1000.0)
    (`/Game/Somewhere/Core/Player/CH_SurvivalCharacter.SERVER Show Talking Widget` (cast `/Game/Somewhere/Core/Player/CH_SurvivalCharacter` (`self.K2_GetPawn`) :!pure true) true)
    (else
      (bind _returnvalue_2 (`UniversalVoiceChat.VoiceChatIsSpeaking`))
      (if _returnvalue_2
        (`UniversalVoiceChat.VoiceChatStopSpeak`)
        (`/Game/Somewhere/Core/Player/CH_SurvivalCharacter.SERVER Show Talking Widget` (cast `/Game/Somewhere/Core/Player/CH_SurvivalCharacter` (`self.K2_GetPawn`) :!pure true) false)))))

(fn `UserConstructionScript`)