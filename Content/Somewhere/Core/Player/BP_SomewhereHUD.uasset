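; BP_SomewhereHUD creates the player's in-game HUD widget once the local player's character is linked.
; On BeginPlay it binds to the Somewhere player controller's character-linked delegate and also fires the handler directly if a character is already linked.
; The handler asynchronously pushes a mobile or desktop HUD class to the UI.Layer.Game layer, then stores the resulting W_HUDBase on the player controller.
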(event `self.ReceiveBeginPlay`
  (bind _returnvalue (`SomewhereStatics.GetSomewherePlayerController` 0))
  (add `SomewherePlayerController.OnPlayerCharacterLinkedDelegate` _returnvalue (`|CreateDelegate` :!event `On Player Character Linked`))
  (`/Engine/EditorBlueprintResources/StandardMacros.IsValid` (`SomewherePlayerController.GetLinkedSomewhereCharacter` _returnvalue)
    (:`Is Valid`
      (`self.On Player Character Linked` null))))

(event `On Player Character Linked`
  (params (SomewhereCharacter :type "SomewhereCharacter Object Reference"))
  (bind _activatablewidget (`AsyncAction_PushWidgetToLayer.PushWidgetToLayerAsync` (struct :`TagName` "UI.Layer.Game") "/Game/Somewhere/UIv2/Widgets/Gameplay/HUD/WM_HUD.WM_HUD_C" "/Game/Somewhere/UIv2/Widgets/Gameplay/HUD/WD_HUD.WD_HUD_C")
    (:`Completed`
      (bind _asw_hudbase (cast `/Game/Somewhere/UIv2/Widgets/Gameplay/HUD/W_HUDBase` _activatablewidget))
      (set `SomewherePlayerController.HUDWidget` _asw_hudbase (`SomewhereStatics.GetSomewherePlayerController` 0)))))

(fn `UserConstructionScript`)