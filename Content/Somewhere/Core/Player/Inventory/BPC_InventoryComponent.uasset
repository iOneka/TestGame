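; Player inventory component that manages item use, pickup, dropping and the held item.
; The server creates main and armor containers, loads starting items from a data table, applies the controller's pouch size and spawns returned items into the world.
; Quickslot keys run UseItem locally then by server RPC, consuming food or toggling server-spawned holdables.
; Armor equip/unequip and swap handling are disconnected; client add/remove handlers send analytics.
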(event `Key|One`
  (params (Key :type "Key Structure"))
  ;[0 0 0] Quickslots
  (:`Pressed`
    (bind _success (`self.Use Item` 0))
    (if _success
      (`self.SERVER Use Item` 0))))

(event `Key|Four`
  (params (Key :type "Key Structure"))
  ;[0 0 0] Quickslots
  (:`Pressed`
    (bind _success (`self.Use Item` 3))
    (if _success
      (`self.SERVER Use Item` 3))))

(event `Key|Two`
  (params (Key :type "Key Structure"))
  ;[0 0 0] Quickslots
  (:`Pressed`
    (bind _success (`self.Use Item` 1))
    (if _success
      (`self.SERVER Use Item` 1))))

(event `Key|Five`
  (params (Key :type "Key Structure"))
  ;[0 0 0] Quickslots
  (:`Pressed`
    (bind _success (`self.Use Item` 4))
    (if _success
      (`self.SERVER Use Item` 4))))

(event `Key|Three`
  (params (Key :type "Key Structure"))
  ;[0 0 0] Quickslots
  (:`Pressed`
    (bind _success (`self.Use Item` 2))
    (if _success
      (`self.SERVER Use Item` 2))))

(event `Key|Six`
  (params (Key :type "Key Structure"))
  ;[0 0 0] Quickslots
  (:`Pressed`
    (bind _success (`self.Use Item` 5))
    (if _success
      (`self.SERVER Use Item` 5))))

(event `self.ReceiveBeginPlay`
  (bind _aspc_survival_controller (cast `/Game/Somewhere/Core/Player/PC_SurvivalController` (`SomewhereCharacter.GetSomewherePlayerController` (`self.Owner as Somewhere Character`)) :!pure true))
  ;[0 0 0] взлом жопы
  (`|ExecutionSequence`
    (:`then_0`
      (`|ExecutionSequence`
        (:`then_0`
          ;[0 0 0] Owner as Character
          (bind _ascharacter (cast `Character` (`self.GetOwner`)))
          (set `self.Owner as Character` _ascharacter)
          (bind _assomewhere_character (cast `SomewhereCharacter` (`self.GetOwner`)))
          (set `self.Owner as Somewhere Character` _assomewhere_character))))
    (:`then_1`
      (`/Engine/EditorBlueprintResources/ActorComponentMacros.Switch Has Authority`
        (:`Authority`
          (`|ExecutionSequence`
            (:`then_0`
              ;[0 0 0] Initialize Inventory
              (`self.Initialize Inventory`)
              (add `ItemContainer.OnItemsSwapped` (`self.Main Container`) (`|CreateDelegate` :!event `On Items Swapped`))
              (add `ItemContainer.OnItemAdded` (`self.Main Container`) (`|CreateDelegate` :!event `On Item Added`))
              (add `ItemContainer.OnItemRemoved` (`self.Main Container`) (`|CreateDelegate` :!event `On Item Removed`))
              (`KismetSystemLibrary.Delay` 1.0)
              (bind _returnvalue (`ItemContainer.ReinitializeWithItemsAndCellSize` (`/Game/Somewhere/Core/Player/PC_SurvivalController.Poach Container` _aspc_survival_controller) (make `InventoryItems` (`|MakeArray` (struct) :!type "InventoryItem Structure")) (`/Game/Somewhere/Core/Player/PC_SurvivalController.Poach Size` _aspc_survival_controller) (`self.Main Container`)))
              (for _array_element (break `InventoryItems` _returnvalue)
                (`|SpawnActorFromClass` "/Game/Somewhere/Core/Other/BP_InventoryItem.BP_InventoryItem_C" (`Actor.GetTransform` (`self.Owner as Somewhere Character`)) "Undefined" "MultiplyWithRoot" null _array_element null)))))))
    (:`then_2`
      (if (`Pawn.IsLocallyControlled` (cast `Character` (`self.GetOwner`) :!pure true))
        (`|ExecutionSequence`
          (:`then_0`
            (`/Engine/EditorBlueprintResources/StandardMacros.IsValid` (`self.Main Container`) :!label _label
              (:`Is Valid`
                (add `ItemContainer.OnItemsSwapped` (`self.Main Container`) (`|CreateDelegate` :!event `On Items Swapped`))
                (add `ItemContainer.OnItemAdded` (`self.Main Container`) (`|CreateDelegate` :!event `On Item Added`))
                (add `ItemContainer.OnItemRemoved` (`self.Main Container`) (`|CreateDelegate` :!event `On Item Removed`)))
              (:`Is Not Valid`
                (`KismetSystemLibrary.Delay` 0.2)
                (goto _label)))))))))

(event `SERVER Use Item`
  (params (Cell :type Integer))
  (`/Game/Somewhere/Core/Libraries/BML_BPC_Somewhere.Switch Has Authority 2`
    (:`Server`
      (`self.Use Item` Cell))))

(event `SERVER Equip Armor`
  (params (`From Cell` :type Integer) (`Armor Type` :type Byte :default 0))
  (`/Game/Somewhere/Core/Libraries/BML_BPC_Somewhere.Switch Has Authority 2`
    (:`Server`
      (`self.Equip Armor` `From Cell` `Armor Type`))))

(event `SERVER Unequip Armor`
  (params (`To Cell` :type Integer) (`Armor Type` :type "EArmorType Enum" :default "Head"))
  (`/Game/Somewhere/Core/Libraries/BML_BPC_Somewhere.Switch Has Authority 2`
    (:`Server`
      (`self.Unequip Armor` `To Cell` `Armor Type`))))

(event `SERVER Pickup Item`
  (params (`Inventory Item` :type "/Game/Somewhere/Core/Other/BP_InventoryItem Object Reference"))
  (`/Game/Somewhere/Core/Libraries/BML_BPC_Somewhere.Switch Has Authority 2`
    (:`Server`
      (`self.Pick Up Item` `Inventory Item`))))

(event `SERVER Drop Item`
  (params (Cell :type Integer))
  (`/Game/Somewhere/Core/Libraries/BML_BPC_Somewhere.Switch Has Authority 2`
    (:`Server`
      (`self.Drop Item` Cell))))

(event `self.ReceiveEndPlay`
  (params (EndPlayReason :type "EEndPlayReason Enum" :default "Destroyed"))
  ;[0 0 0] взлом жопы
  (`|ExecutionSequence`
    (:`then_0`
      (`|ExecutionSequence`
        (:`then_0`
          ;[0 0 0] Удаляем оружие в руках
          (bind _current_holdable (`self.Current Holdable`)
            (:`then`
              (`Actor.K2_DestroyActor` _current_holdable))
            (:`else`)))))
    (:`then_2`
      (if (`Pawn.IsLocallyControlled` (cast `Character` (`self.GetOwner`) :!pure true))
        (`|ExecutionSequence`)))))

(fn `Drop Item`
  (params (Cell :type Integer))
  (locals (`L Items` :type "InventoryItem Structure"))
  (bind _returnvalue (`self.GetOwner`))
  (bind _output_get (set `local.L Items` (`ItemContainer.GetCell` (`self.Main Container`) Cell)))
  (`ItemContainer.RemoveItemFromCell` (`self.Main Container`) _output_get (`local.Cell`))
  (`/Engine/EditorBlueprintResources/ActorComponentMacros.Switch Has Authority`
    (:`Authority`
      (`|SpawnActorFromClass` "/Game/Somewhere/Core/Other/BP_InventoryItem.BP_InventoryItem_C" (`KismetMathLibrary.MakeTransform` (+ (`Actor.K2_GetActorLocation` _returnvalue) (* (`Actor.GetActorForwardVector` _returnvalue) 50.0))) "Undefined" "OverrideRootScale" null (`local.L Items`) null)
      (bind _current_holdable (`self.Current Holdable`)
        (:`then`
          (`Actor.K2_DestroyActor` _current_holdable))
        (:`else`)))))

(fn `Equip Armor`
  (params (`From Cell` :type Integer) (`Armor Type` :type Byte :default 0))
  (returns (Success :type Boolean))
  (locals (`L Item` :type " Structure") (`L Item Definition` :type " Structure")))

(fn `Equip Holdable`)

(fn `Initialize Inventory`
  (`|ExecutionSequence`
    (:`then_0`
      (bind _returnvalue (`|AddComponentByClass` (`self.Owner as Character`) "/Script/SOMEWHERE.ItemContainer"))
      (set `self.Main Container` _returnvalue)
      (bind _returnvalue_2 (`|AddComponentByClass` (`self.Owner as Character`) "/Script/SOMEWHERE.ItemContainer"))
      (set `self.Armor Container` _returnvalue_2))
    (:`then_1`
      ;[0 0 0] Предметы
      (`ItemContainer.Initialize` (`self.Main Container`) 30)
      (bind _returnvalue_3 (`|GetDataTableRow` "/Game/Somewhere/Core/Player/Inventory/DT_StartingItems.DT_StartingItems" (`PlatformStatics.GetDeveloperName`))
        (:`then`
          (for _array_element (`.Items` (break `InventoryItems` _returnvalue_3))
            (`ItemContainer.AddItem` (`self.Main Container`) _array_element)))
        (:`RowNotFound`
          (bind _returnvalue_4 (`|GetDataTableRow` "/Game/Somewhere/Core/Player/Inventory/DT_StartingItems.DT_StartingItems" "default")
            (:`then`
              (for _array_element_2 (`.Items` (break `InventoryItems` _returnvalue_4))
                (`ItemContainer.AddItem` (`self.Main Container`) _array_element_2)))))))))

(fn `On Item Added`
  (params (Container :type "ItemContainer Object Reference") (Item :type "InventoryItem Structure") (ToCells :type "Array of Integer (by ref)"))
  (bind (_id _amount) (break `InventoryItem` Item))
  (`/Engine/EditorBlueprintResources/ActorComponentMacros.Switch Has Authority`
    (:`Remote`
      (`/Game/Somewhere/Core/Subsystems/AnalyticService.Send Event` (subsystem `/Game/Somewhere/Core/Subsystems/AnalyticService`) "Item Added" (`KismetStringLibrary.Conv_NameToString` _id) (`KismetStringLibrary.Conv_IntToString` _amount) "" "")
      (return))))

(fn `On Item Removed`
  (params (Container :type "ItemContainer Object Reference") (Item :type "InventoryItem Structure") (FromCells :type "Array of Integer (by ref)"))
  (bind (_id _amount) (break `InventoryItem` Item))
  (`/Engine/EditorBlueprintResources/ActorComponentMacros.Switch Has Authority`
    (:`Remote`
      (`/Game/Somewhere/Core/Subsystems/AnalyticService.Send Event` (subsystem `/Game/Somewhere/Core/Subsystems/AnalyticService`) "Item Removed" (`KismetStringLibrary.Conv_NameToString` _id) (`KismetStringLibrary.Conv_IntToString` _amount) "" "")
      (return))))

(fn `On Items Swapped`
  (params (FromCell :type Integer) (FromContainer :type "ItemContainer Object Reference") (ToCell :type Integer) (ToContainer :type "ItemContainer Object Reference")))

(fn `Pick Up Item`
  (params (`Inventory Item` :type "/Game/Somewhere/Core/Other/BP_InventoryItem Object Reference"))
  (returns (Success :type Boolean))
  (locals (`L Item Data` :type " Structure") (`L Free Space` :type Integer :default 0) (`L Inventory Item` :type "InventoryItem Structure"))
  (bind (_l_inventory_item_id _l_inventory_item_amount _l_inventory_item_cell _l_inventory_item_custominteger _l_inventory_item_durability _l_inventory_item_additionaldata) (break `InventoryItem` (`local.L Inventory Item`)))
  (bind (_l_inventory_item_id_2 _l_inventory_item_amount_2 _l_inventory_item_cell_2 _l_inventory_item_custominteger_2 _l_inventory_item_durability_2 _l_inventory_item_additionaldata_2) (break `InventoryItem` (`local.L Inventory Item`)))
  (`/Engine/EditorBlueprintResources/StandardMacros.IsValid` `Inventory Item`
    (:`Is Valid`
      (set `local.L Inventory Item` (`/Game/Somewhere/Core/Other/BP_InventoryItem.Inventory Item` (`local.Inventory Item`)))
      ;[0 0 0] Сколько места для этого предмета есть у нас в инвентаре?
      (bind _output_get (set `local.L Free Space` (`ItemContainer.FindFreeSpaceForItem` (`self.Main Container`) (`.ID` (break `InventoryItem` (`local.L Inventory Item`))))))
      (if (> _output_get 0)
        ;[0 0 0] Покладываем предмет к себе
        (bind _returnvalue (`ItemContainer.AddItem` (`self.Main Container`) (make `InventoryItem` _l_inventory_item_id_2 (`KismetMathLibrary.Clamp` (`local.L Free Space`) 0 _l_inventory_item_amount_2) _l_inventory_item_cell_2 _l_inventory_item_custominteger_2 _l_inventory_item_durability_2 _l_inventory_item_additionaldata_2)))
        (if _returnvalue
          ;[0 0 0] Остатки, которые не поместились
          (if (>= (`local.L Free Space`) (`.Amount` (break `InventoryItem` (`local.L Inventory Item`))))
            (`Actor.K2_DestroyActor` (`local.Inventory Item`))
            (return true)
            (else
              (set `/Game/Somewhere/Core/Other/BP_InventoryItem.Inventory Item` (make `InventoryItem` _l_inventory_item_id (- _l_inventory_item_amount (`local.L Free Space`)) _l_inventory_item_cell _l_inventory_item_custominteger _l_inventory_item_durability _l_inventory_item_additionaldata) (`local.Inventory Item`))))
          (else
            (return false)))
        (else
          (`GameplayMessageSubsystem.K2_BroadcastMessage` (subsystem `GameplayMessageSubsystem`) (struct :`TagName` "GameplayMessage.NotEnoughSpace") (make `EmptyPayload`))
          (return false))))))

(fn `Unequip Armor`
  (params (`To Cell` :type Integer) (`Armor Type` :type "EArmorType Enum" :default "Head"))
  (returns (Success :type Boolean))
  (locals (`Armor Item` :type " Structure") (`Inventory Item` :type " Structure")))

(fn `Use Item`
  (params (Cell :type Integer))
  (returns (Success :type Boolean))
  (locals (`L Item2` :type "InventoryItem Structure") (`L Item Definition2` :type "ItemDefinition Structure") (`L Item Properties` :type "ItemProperties Structure"))
  (bind _owner_as_character (`self.Owner as Character`))
  (bind (_id _amount _cell _custominteger _durability _additionaldata) (break `InventoryItem` (`local.L Item2`)))
  (bind _health_component (`/Game/Somewhere/Core/Libraries/BFL_Somewhere.Get Health Component` (`self.Owner as Character`)))
  (bind ((`Hunger` _hunger) (`Thirst` _thirst)) (break `ItemProperties_Food` (`.Food` (break `ItemProperties` (`local.L Item Properties`)))))
  ;[0 0 0] Предмет
  (if (and (`ItemContainer.IsValidCellIndex` (`self.Main Container`) (`local.Cell`)) (`.ReturnValue` (`ItemContainer.GetCell` (`self.Main Container`) (`local.Cell`))))
    ;[0 0 0] Игрок
    (if (`/Game/Somewhere/Core/Player/Health/BPC_HealthComponent.Is Alive` (`/Game/Somewhere/Core/Libraries/BFL_Somewhere.Get Health Component` (`self.Owner as Character`)))
      (bind _output_get (set `local.L Item2` (`ItemContainer.GetCell` (`self.Main Container`) (`local.Cell`))))
      (bind _output_get_2 (set `local.L Item Definition2` (`InventoryStatics.GetItemDefinitionFromItem` _output_get)))
      (set `local.L Item Properties` (`.Properties` (break `ItemDefinition` _output_get_2)))
      (switch `EItemType` (`.Type` (break `ItemDefinition` (`local.L Item Definition2`)))
        (:`Food`
          ;[1 0.3531 0 0.1] Удаляем одно яблочко
          (bind _returnvalue (`ItemContainer.RemoveItemAmountFromCell` (`self.Main Container`) (`local.Cell`) 1))
          (if _returnvalue
            ;[1 0.839 0 0.1] Хаваем его
            (`HealthComponent.SetHunger` _health_component (+ _hunger (`HealthComponent.GetHunger` _health_component)))
            (`HealthComponent.SetThirst` _health_component (+ _thirst (`HealthComponent.GetThirst` _health_component)))
            ;[0.005 1 0] да
            (`self.On Item Used` (`local.Cell`) (make `InventoryItem` _id 1 _cell _custominteger _durability _additionaldata))
            (return true)
            (else
              ;;[1 0 0] фак
              (return false))))
        (:`Clothing`)
        (:`Weapons`
          _)
        (:`Medicals`
          _)
        (:`Props`
          _))
      ;[0 0 0] Оружия можно брать в руки только из хотбара
      (if (< (`local.Cell`) 6)
        ;[0 0 0] Валидное оружие?
        (if (`KismetSystemLibrary.IsValidSoftClassReference` (`.HoldableClass` (break `ItemProperties_Weapon` (`.Weapon` (break `ItemProperties` (`local.L Item Properties`))))))
          ;[0 0 0] Есть оружие в руках?
          (`/Engine/EditorBlueprintResources/StandardMacros.IsValid` (`self.Current Holdable`)
            (:`Is Valid`
              ;[0 0 0] Юзаем то же оружие, которое в руках?
              (if (== (`/Game/Somewhere/Core/Holdable/BP_Holdable.Cell Item` (`self.Current Holdable`)) (`local.Cell`))
                ;[0 0 0] Прячем
                (`Actor.K2_DestroyActor` (`self.Current Holdable`))
                (set `self.Current Holdable` null)
                (else
                  ;[0 0 0] Прячем
                  (`Actor.K2_DestroyActor` (`self.Current Holdable`))
                  (set `self.Current Holdable` null)
                  (`/Engine/EditorBlueprintResources/ActorComponentMacros.Switch Has Authority` :!label _label
                    (:`Authority`
                      (bind _returnvalue_2 (`KismetSystemLibrary.LoadClassAsset_Blocking` (`.HoldableClass` (break `ItemProperties_Weapon` (`.Weapon` (break `ItemProperties` (`local.L Item Properties`)))))))
                      ;[0 0 0] Показываем
                      (bind _asbp_holdable (castclass `/Game/Somewhere/Core/Holdable/BP_Holdable` _returnvalue_2))
                      (bind _returnvalue_3 (`|SpawnActorFromClass` _asbp_holdable (`KismetMathLibrary.MakeTransform` (0.0 0.0 0.0)) "AlwaysSpawn" "SelectDefaultAtRuntime" _owner_as_character (`local.Cell`) (`local.L Item2`) _owner_as_character))
                      (set `self.Current Holdable` _returnvalue_3)
                      (return true))
                    (:`Remote`
                      (return true))))))
            (:`Is Not Valid`
              (goto _label)))
          (else
            ;;[1 0 0] фак
            (return false))))
      (else
        ;;[1 0 0] дабл фак
        (return false)))
    (else
      ;[0 0 0] Мб мы хотим убрать оружие, тыкнув по пустой ячейке хотбара
      (if (< (`local.Cell`) 6)
        (`/Engine/EditorBlueprintResources/StandardMacros.IsValid` (`self.Current Holdable`)
          (:`Is Valid`
            (`Actor.K2_DestroyActor` (`self.Current Holdable`))
            (set `self.Current Holdable` null)
            (return true))
          (:`Is Not Valid`
            _)))
      ;[1 0 0] фак
      (return false))))