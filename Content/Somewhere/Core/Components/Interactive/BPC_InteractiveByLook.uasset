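; Interactive component that detects when a nearby character's player is looking at it and signals look start and end.
; BeginPlay spawns a pawn-only proximity sphere and sets child shapes to the Interactable object type, ignoring all channels.
; Overlap, handled on server and locally controlled client, runs a looping timer instead of Tick for one tracked character.
; Each timer step object-traces from the camera against those shapes; leaving the sphere also ends the look.
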(event `On Distance Sphere Begin Overlap`
  (params (OverlappedComponent :type "PrimitiveComponent Object Reference") (OtherActor :type "Actor Object Reference") (OtherComp :type "PrimitiveComponent Object Reference") (OtherBodyIndex :type Integer) (bFromSweep :type Boolean) (SweepResult :type "HitResult Structure (by ref)"))
  (if (`self.IsActive`)
    (`/Engine/EditorBlueprintResources/StandardMacros.IsValid` OtherActor
      (:`Is Valid`
        ;[0 0 0] Ограничиваем ивент до сервера и локального клиента
        (bind _assomewhere_character (cast `SomewhereCharacter` OtherActor))
        (`/Game/Somewhere/Core/Libraries/BML_BPC_Somewhere.Switch Has Authority 2`
          (:`Server`
            ;[0 0 0] Кто
            (bind _output_get (set `self.Overlapped Character` _assomewhere_character :!label _label))
            (bind _asplayer_controller (cast `PlayerController` (`Pawn.GetController` _output_get)))
            (set `self.Overlapped Player Controller` _asplayer_controller)
            (set `self.Is Looking` false)
            ;[0 0 0] Запускаем тик
            (bind _returnvalue (`KismetSystemLibrary.K2_SetTimerDelegate` (`|CreateDelegate` :!event `Line Trace Timer`) 0.1 true))
            (set `self.Line Trace Timer Handle` _returnvalue))
          (:`Standalone`
            (if (`Pawn.IsLocallyControlled` _assomewhere_character) :!label _label_2
              (goto _label)))
          (:`Client`
            (goto _label_2)))))))

(event `On Distance Sphere End Overlap`
  (params (OverlappedComponent :type "PrimitiveComponent Object Reference") (OtherActor :type "Actor Object Reference") (OtherComp :type "PrimitiveComponent Object Reference") (OtherBodyIndex :type Integer))
  (if (`self.IsActive`)
    (`/Engine/EditorBlueprintResources/StandardMacros.IsValid` OtherActor
      (:`Is Valid`
        ;[0 0 0] Ограничиваем ивент до сервера и локального клиента
        (bind _assomewhere_character (cast `SomewhereCharacter` OtherActor))
        (`/Game/Somewhere/Core/Libraries/BML_BPC_Somewhere.Switch Has Authority 2`
          (:`Server`
            ;[0 0 0] Выключаем тик
            (`KismetSystemLibrary.K2_ClearAndInvalidateTimerHandle` (`self.Line Trace Timer Handle`) :!label _label_3)
            ;[0 0 0] Если игрок вышел из сферы при этом смотря на объект
            (if (`self.Is Looking`)
              (`self.On Player Interactive Look Ended` (`self.Overlapped Character`))
              ;[0 0 0] Никто
              (set `self.Overlapped Character` null)
              (set `self.Overlapped Player Controller` null)
              (set `self.Is Looking` false)))
          (:`Standalone`
            (if (`Pawn.IsLocallyControlled` _assomewhere_character) :!label _label_4
              (goto _label_3)))
          (:`Client`
            (goto _label_4)))))))

(event `self.ReceiveBeginPlay`
  (bind _distance_sphere (`self.Distance Sphere`))
  (`|ExecutionSequence`
    (:`then_0`
      ;[0 0 0] Спавним сферу чтобы узнать рядом ли игрок или нет
      (bind _returnvalue (`|AddComponentByClass` (`self.GetOwner`) "/Script/Engine.SphereComponent" false (`KismetMathLibrary.MakeTransform` (`self.Distance Sphere Location`))))
      (bind _output_get (set `self.Distance Sphere` _returnvalue))
      (`SphereComponent.SetSphereRadius` _output_get (`self.Distance Sphere Radius`) true)
      ;[0 0 0] Реагируем только на пешек, всё остальное игнорим
      (`PrimitiveComponent.SetCollisionObjectType` _distance_sphere "ECC_WorldDynamic")
      (`PrimitiveComponent.SetCollisionResponseToAllChannels` _distance_sphere "ECR_Ignore")
      (`PrimitiveComponent.SetCollisionResponseToChannel` _distance_sphere "ECC_Pawn" "ECR_Overlap")
      (add `PrimitiveComponent.OnComponentBeginOverlap` (`self.Distance Sphere`) (`|CreateDelegate` :!event `On Distance Sphere Begin Overlap`))
      (add `PrimitiveComponent.OnComponentEndOverlap` (`self.Distance Sphere`) (`|CreateDelegate` :!event `On Distance Sphere End Overlap`)))
    (:`then_1`
      ;[0 0 0] Берем все коллизии под этим компонентом
      (`KismetArrayLibrary.Array_Clear` (`self.Interactive Collisions`))
      (for _array_element (`self.GetChildrenComponents` true)
        (bind _asshape_component (cast `ShapeComponent` _array_element))
        (`KismetArrayLibrary.Array_Add` (`self.Interactive Collisions`) _asshape_component)
        ;[0 0 0] Ставим им тип объекта Interactable, но игнорим всё (в функции LineTrace будем трейсить по типу объекта)
        (`PrimitiveComponent.SetCollisionObjectType` _asshape_component "ECC_GameTraceChannel4")
        (`PrimitiveComponent.SetCollisionResponseToAllChannels` _asshape_component "ECR_Ignore")))
    (:`then_2`
      ;[0 0 0] Если игрок уже находится рядом, вручную раним ивент
      (for _array_element_2 (`PrimitiveComponent.GetOverlappingActors` (`self.Distance Sphere`) "/Script/SOMEWHERE.SomewhereCharacter")
        (`self.On Distance Sphere Begin Overlap` null _array_element_2 null 0 false (`GameplayStatics.MakeHitResult` false))))))

(event `Line Trace Timer`
  (if (`self.IsActive`)
    (bind _hit (`self.Line Trace`))
    (if _hit
      (if (not (`self.Is Looking`))
        (set `self.Is Looking` true)
        (`self.On Player Interactive Look Started` (`self.Overlapped Character`)))
      (elif (`self.Is Looking`)
        (set `self.Is Looking` false)
        (`self.On Player Interactive Look Ended` (`self.Overlapped Character`))))
    (else
      (`KismetSystemLibrary.K2_ClearAndInvalidateTimerHandle` (`self.Line Trace Timer Handle`)))))

(event `self.ReceiveEndPlay`
  (params (EndPlayReason :type "EEndPlayReason Enum" :default "Destroyed"))
  (bind _distance_sphere (`self.Distance Sphere`))
  ;[0 0 0] Во время дестроя вызывается ивент 'End Overlap', нужно отписаться чтобы не было путаницы
  (clear `PrimitiveComponent.OnComponentBeginOverlap` _distance_sphere)
  (clear `PrimitiveComponent.OnComponentEndOverlap` _distance_sphere))

(fn `Line Trace`
  (returns (Hit :type Boolean))
  (locals (`L Start` :type "Vector Structure" :default (0.0 0.0 0.0)) (`L End` :type "Vector Structure") (`L Actors to Ignore` :type "Array of Character Object Reference"))
  (`self.Overlapped Character`
    (:`then`
      (`self.Overlapped Player Controller`
        (:`then`
          (`|ExecutionSequence`
            (:`then_0`
              ;[0 0 0] Начало от камеры
              (set `local.L Start` (`Actor.K2_GetActorLocation` (`PlayerController.PlayerCameraManager` (`self.Overlapped Player Controller`))))
              ;[0 0 0] Конец куда смотрим
              (set `local.L End` (+ (`local.L Start`) (* 1000.0 (`Actor.GetActorForwardVector` (`PlayerController.PlayerCameraManager` (`self.Overlapped Player Controller`))))))
              (set `local.L Actors to Ignore` (`|MakeArray` (`self.Overlapped Character`))))
            (:`then_1`
              (bind (_outhit _returnvalue) (`KismetSystemLibrary.LineTraceSingleForObjects` (`local.L Start`) (`local.L End`) (`|MakeArray` "ObjectTypeQuery8" :!type "EObjectTypeQuery Enum") false (`local.L Actors to Ignore`) "None" false (struct :`R` 1.0 :`A` 1.0) (struct :`G` 1.0 :`A` 1.0) 0.1))
              (if _returnvalue
                (bind _asshape_component (cast `ShapeComponent` (`.HitComponent` (`GameplayStatics.BreakHitResult` _outhit)))
                  (:`then`
                    (return (`KismetArrayLibrary.Array_Contains` (`self.Interactive Collisions`) _asshape_component)))
                  (:`CastFailed`
                    (return false)))
                (else
                  (return false))))))
        (:`else`
          (return false))))
    (:`else`
      (return false))))