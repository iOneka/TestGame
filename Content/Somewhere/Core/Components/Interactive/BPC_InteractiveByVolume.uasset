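; Interactive component that signals when a SomewhereCharacter enters or exits the volume formed by its child shape components.
; At BeginPlay it makes those shapes overlap only Pawns and binds their overlap events, handled on the server and for locally controlled characters.
; It tracks one character, firing enter on first overlap and exit once no shape contains them.
; Existing overlaps are replayed at BeginPlay and on activation; the forward-visibility trace is unused.
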(event `On Collisions Begin Overlap`
  (params (OverlappedComponent :type "PrimitiveComponent Object Reference") (OtherActor :type "Actor Object Reference") (OtherComp :type "PrimitiveComponent Object Reference") (OtherBodyIndex :type Integer) (bFromSweep :type Boolean) (SweepResult :type "HitResult Structure (by ref)"))
  (if (`self.IsActive`)
    ;[0 0 0] Ограничиваем ивент до сервера и локального клиента
    (bind _assomewhere_character (cast `SomewhereCharacter` OtherActor))
    (`/Game/Somewhere/Core/Libraries/BML_BPC_Somewhere.Switch Has Authority 2`
      (:`Server`
        ;[0 0 0] Если персонаж впервые зашёл в коллизии
        (`/Engine/EditorBlueprintResources/StandardMacros.IsValid` (`self.Overlapped Character`) :!label _label
          (:`Is Not Valid`
            (set `self.Overlapped Character` _assomewhere_character)
            (`self.On Player Entered Interactive Volume` (`self.Overlapped Character`)))))
      (:`Standalone`
        (if (`Pawn.IsLocallyControlled` _assomewhere_character) :!label _label_2
          (goto _label)))
      (:`Client`
        (goto _label_2)))))

(event `On Collisions End Overlap`
  (params (OverlappedComponent :type "PrimitiveComponent Object Reference") (OtherActor :type "Actor Object Reference") (OtherComp :type "PrimitiveComponent Object Reference") (OtherBodyIndex :type Integer))
  (if (`self.IsActive`)
    ;[0 0 0] Ограничиваем ивент до сервера и локального клиента
    (bind _assomewhere_character (cast `SomewhereCharacter` OtherActor))
    (`/Game/Somewhere/Core/Libraries/BML_BPC_Somewhere.Switch Has Authority 2`
      (:`Server`
        ;[0 0 0] Если персонаж вышел из всех коллизий
        (set `self.Overlapped Character` _assomewhere_character :!label _label_3)
        (if (not (`self.Any Collision Contains Player`))
          (`self.On Player Exited Interactive Volume` (`self.Overlapped Character`))
          (set `self.Overlapped Character` null)))
      (:`Standalone`
        (if (`Pawn.IsLocallyControlled` _assomewhere_character) :!label _label_4
          (goto _label_3)))
      (:`Client`
        (goto _label_4)))))

(event `self.ReceiveBeginPlay`
  (`|ExecutionSequence`
    (:`then_0`
      ;[0 0 0] Берем все коллизии под этим компонентом
      (`KismetArrayLibrary.Array_Clear` (`self.Interactive Collisions`))
      (for _array_element (`self.GetChildrenComponents` true)
        (bind _asshape_component (cast `ShapeComponent` _array_element))
        (`KismetArrayLibrary.Array_Add` (`self.Interactive Collisions`) _asshape_component)
        ;[0 0 0] Реагируем только на пешек, всё остальное игнорим
        (`PrimitiveComponent.SetCollisionObjectType` _asshape_component "ECC_WorldDynamic")
        (`PrimitiveComponent.SetCollisionResponseToAllChannels` _asshape_component "ECR_Ignore")
        (`PrimitiveComponent.SetCollisionResponseToChannel` _asshape_component "ECC_Pawn" "ECR_Overlap")
        (add `PrimitiveComponent.OnComponentBeginOverlap` _asshape_component (`|CreateDelegate` :!event `On Collisions Begin Overlap`))
        (add `PrimitiveComponent.OnComponentEndOverlap` _asshape_component (`|CreateDelegate` :!event `On Collisions End Overlap`))))
    (:`then_2`
      ;[0 0 0] Если игрок уже находится рядом, вручную раним ивент
      (`self.Force Update Overlaps`))
    (:`then_3`
      (add `self.OnComponentActivated` (`|CreateDelegate` :!event `On Component Activated`))
      (add `self.OnComponentDeactivated` (`|CreateDelegate` :!event `On Component Deactivated`)))))

(event `On Component Activated` :!signature `self.OnComponentActivated`
  (params (Component :type "ActorComponent Object Reference") (bReset :type Boolean))
  (`self.Force Update Overlaps`))

(event `On Component Deactivated` :!signature `self.OnComponentDeactivated`
  (params (Component :type "ActorComponent Object Reference")))

(event `self.ReceiveEndPlay`
  (params (EndPlayReason :type "EEndPlayReason Enum" :default "Destroyed"))
  ;[0 0 0] Во время дестроя вызывается ивент 'End Overlap', нужно отписаться чтобы не было путаницы
  (for _array_element (`self.Interactive Collisions`)
    (clear `PrimitiveComponent.OnComponentBeginOverlap` _array_element)
    (clear `PrimitiveComponent.OnComponentEndOverlap` _array_element)))

(fn `Any Collision Contains Player`
  (returns (Contains :type Boolean))
  (for _array_element (`self.Interactive Collisions`)
    (`/Engine/EditorBlueprintResources/StandardMacros.IsValid` _array_element
      (:`Is Valid`
        (if (`KismetArrayLibrary.Array_Contains` (`PrimitiveComponent.GetOverlappingActors` _array_element "/Script/SOMEWHERE.SomewhereCharacter") (`self.Overlapped Character`))
          (return true)))))
  (return false))

(fn `Force Update Overlaps`
  (for _array_element (`self.Interactive Collisions`)
    (for _array_element_2 (`PrimitiveComponent.GetOverlappingActors` _array_element "/Script/SOMEWHERE.SomewhereCharacter")
      (`self.On Collisions Begin Overlap` null _array_element_2 null 0 false (`GameplayStatics.MakeHitResult` false)))))

(fn `Player Has Forward Visibility`
  (returns (`Can Interact` :type Boolean))
  (locals (`array elem` :type "StaticMeshComponent Object Reference")))