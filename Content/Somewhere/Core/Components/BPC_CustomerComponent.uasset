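; Customer component that handles shop purchases paid with inventory items or PlayFab virtual currency.
; Item purchases read DataTable rows, check and remove price items, then add the bought item, spawning a pickup if adding fails.
; Currency purchases call PlayFab's SpendMoney function, grant the item on success and refresh Golden Caps.
; Clients apply purchases locally, then have the server rerun the same flow, including the SpendMoney call.
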(event `ForGameItemsPurchase`
  (params (PlayerCharacter :type "Actor Object Reference") (RowName :type Name) (DataTable :type "DataTable Object Reference") (CountToBuy :type Integer))
  (bind _inventory_component (`/Game/Somewhere/Core/Libraries/BFL_Somewhere.Get Inventory Component` PlayerCharacter))
  (bind _main_container (`/Game/Somewhere/Core/Player/Inventory/BPC_InventoryComponent.Main Container` _inventory_component))
  ;[1 1 1] NE RM
  (bind _returnvalue (`|GetDataTableRow` DataTable RowName)
    (:`then`
      (set `self.PriceItemsAmountError` false)
      (bind (_buyingitemid _buyingitemamount _priceitems) (break `/Game/Somewhere/Core/Data/Structures/S_PurchaceRequiement` _returnvalue))
      (for _array_element _priceitems
        (bind (_item _itemcount) (break `/Game/Somewhere/Core/Data/Structures/S_PurchaseItem` _array_element))
        (bind _returnvalue_2 (`|GetDataTableRow` (break `DataTableRowHandle` _item) (`.RowName` (break `DataTableRowHandle` _item)))
          (:`then`
            (if (> (* CountToBuy _itemcount) (`ItemContainer.GetItemAmount` (`/Game/Somewhere/Core/Player/Inventory/BPC_InventoryComponent.Main Container` _inventory_component) (`.ID` (break `ItemDefinition` _returnvalue_2))))
              (set `self.PriceItemsAmountError` true)
              (break)))))
      (if (`self.PriceItemsAmountError`)
        (`KismetSystemLibrary.PrintString` "Ne hvataet predmetov")
        (else
          (for _array_element_2 _priceitems
            (bind (_item_2 _itemcount_2) (break `/Game/Somewhere/Core/Data/Structures/S_PurchaseItem` _array_element_2))
            (bind _returnvalue_3 (`|GetDataTableRow` (break `DataTableRowHandle` _item_2) (`.RowName` (break `DataTableRowHandle` _item_2)))
              (:`then`
                (bind _output_get (set `self.TempItemAmount` (* _itemcount_2 CountToBuy)))
                (bind _output_get_2 (set `self.Cells` (`ItemContainer.FindAllCellsWithItem` _main_container (`.ID` (break `ItemDefinition` _returnvalue_3)))))
                (for _array_element_3 _output_get_2
                  (`ItemContainer.RemoveItemAmountFromCell` _main_container _array_element_3 _output_get)
                  (bind _output_get_3 (set `self.TempItemAmount` (- _output_get (`.Amount` (break `InventoryItem` (`ItemContainer.GetCell` _main_container _array_element_3))))))
                  (if (not (> _output_get_3 0))
                    (break))))))
          (bind (_datatable _rowname) (break `DataTableRowHandle` _buyingitemid))
          (bind _returnvalue_4 (`|GetDataTableRow` _datatable _rowname)
            (:`then`
              (bind _inventoryitem (make `InventoryItem` (`.ID` (break `ItemDefinition` _returnvalue_4)) (* _buyingitemamount CountToBuy)))
              (bind _returnvalue_5 (`ItemContainer.AddItem` _main_container _inventoryitem))
              (if (not _returnvalue_5)
                ;;[1 0 0] DROP ITEM
                (`|SpawnActorFromClass` "/Game/Somewhere/Core/Other/BP_InventoryItem.BP_InventoryItem_C" (`Actor.GetTransform` PlayerCharacter) "Undefined" "MultiplyWithRoot" null _inventoryitem null))
              (`/Game/Somewhere/Core/Libraries/BML_BPC_Somewhere.Switch Has Authority 2`
                (:`Client`
                  (`self.ServerForGameItemsPurchase` PlayerCharacter RowName DataTable CountToBuy))))))))))

(event `ClientForGameItemsPurchase`
  (params (PlayerCharacter :type "Actor Object Reference") (RowName :type Name) (DataTable :type "DataTable Object Reference") (CountToBuy :type Integer))
  ;[1 1 1] Comment
  (`self.ForGameItemsPurchase` PlayerCharacter RowName DataTable CountToBuy))

(event `ServerForGameItemsPurchase`
  (params (PlayerCharacter :type "Actor Object Reference") (RowName :type Name) (DataTable :type "DataTable Object Reference") (CountToBuy :type Integer))
  ;[1 1 1] Comment
  (`self.ForGameItemsPurchase` PlayerCharacter RowName DataTable CountToBuy))

(event `ServerForVCItemPurchase`
  (params (PlayerCharacter :type "Actor Object Reference") (RowName :type Name) (DataTable :type "DataTable Object Reference") (CountToBuy :type Integer))
  ;[1 1 1] Comment
  (`self.ForVCItemPurchase` PlayerCharacter RowName DataTable CountToBuy))

(event `ClientForVCItemsPurchase`
  (params (PlayerCharacter :type "Actor Object Reference") (RowName :type Name) (DataTable :type "DataTable Object Reference") (CountToBuy :type Integer))
  ;[1 1 1] Comment
  (`self.ForVCItemPurchase` PlayerCharacter RowName DataTable CountToBuy))

(event `SpendMoneySuccess`
  (params (result :type "CloudScriptExecuteFunctionResult Structure") (customData :type "Object Object Reference"))
  ;[1 1 1] Comment
  (`KismetSystemLibrary.PrintString` (`PlayFabJsonObject.GetStringField` result_FunctionResult "success"))
  (if (`PlayFabJsonObject.GetBoolField` result_FunctionResult "success")
    (bind _asch_survival_character (cast `/Game/Somewhere/Core/Player/CH_SurvivalCharacter` (stale `ForVCItemPurchase` PlayerCharacter) :!pure true))
    (bind _inventoryitem (make `InventoryItem` (`.ID` (break `ItemDefinition` (stale `ForVCItemPurchase` _returnvalue_2))) (* (`.BuyingItemAmount_20_06C593B5477881A605C0B891124F5617` (break `/Game/Somewhere/Core/Data/Structures/S_PurchaceRequiement` (stale `ForVCItemPurchase` _returnvalue))) (stale `ForVCItemPurchase` CountToBuy))))
    (bind _returnvalue (`ItemContainer.AddItem` (`/Game/Somewhere/Core/Player/Inventory/BPC_InventoryComponent.Main Container` (`/Game/Somewhere/Core/Libraries/BFL_Somewhere.Get Inventory Component` _asch_survival_character)) _inventoryitem))
    (`|ExecutionSequence`
      (:`then_0`
        (if (not _returnvalue)
          ;;[1 0 0] DROP ITEM
          (`|SpawnActorFromClass` "/Game/Somewhere/Core/Other/BP_InventoryItem.BP_InventoryItem_C" (`Actor.GetTransform` _asch_survival_character) "Undefined" "MultiplyWithRoot" null _inventoryitem null))
        (`/Game/Somewhere/Core/Libraries/BML_BPC_Somewhere.Switch Has Authority 2`
          (:`Client`
            (`self.ServerForVCItemPurchase` (stale `ForVCItemPurchase` PlayerCharacter) (stale `ForVCItemPurchase` RowName) (stale `ForVCItemPurchase` DataTable) (stale `ForVCItemPurchase` CountToBuy)))))
      (:`then_1`
        (`/Game/Somewhere/Core/Subsystems/PlayFabService.Get Golden Caps` (subsystem `/Game/Somewhere/Core/Subsystems/PlayFabService`))))))

(event `SendPlayfabId_TEMP`
  (params (InString :type String))
  ;[1 0 0] TEMP
  (set `self.TEMPPLAYFABID` InString))

(event `ForVCItemPurchase`
  (params (PlayerCharacter :type "Actor Object Reference") (RowName :type Name) (DataTable :type "DataTable Object Reference") (CountToBuy :type Integer))
  ;[1 1 1] Comment
  (bind _returnvalue (`|GetDataTableRow` DataTable RowName)
    (:`then`
      (bind (_buyingitemid _buyingitemamount _priceitems _vc _amountvc) (break `/Game/Somewhere/Core/Data/Structures/S_PurchaceRequiement` _returnvalue))
      (bind (_datatable _rowname) (break `DataTableRowHandle` _buyingitemid))
      (bind _returnvalue_2 (`|GetDataTableRow` _datatable _rowname)
        (:`then`
          (if _vc
            (bind _output_get (set `self.Request Function Parameter` (`PlayFabJsonObject.ConstructJsonObject`)))
            (`PlayFabJsonObject.SetStringField` _output_get "userId" (`SomewherePlayerState.PlayFabID` (`SomewhereCharacter.GetSomewherePlayerState` (cast `/Game/Somewhere/Core/Player/CH_SurvivalCharacter` PlayerCharacter :!pure true))))
            (`PlayFabJsonObject.SetStringField` _output_get "gc" (`KismetStringLibrary.Conv_IntToString` (* _amountvc CountToBuy)))
            (`PlayFabCloudScriptAPI.ExecuteFunction` (make `CloudScriptExecuteFunctionRequest` null null "SpendMoney" _output_get) (delegate `SpendMoneySuccess`) (delegate `SpendMoneyFail`))))))))

(event `SpendMoneyFail`
  (params (error :type "PlayFabError Structure") (customData :type "Object Object Reference"))
  ;[1 1 1] Comment
  (`KismetSystemLibrary.PrintString` (`KismetStringLibrary.Concat_StrStr` (`KismetStringLibrary.Conv_BoolToString` error_hasError) (`KismetStringLibrary.Conv_IntToString` error_ErrorCode) error_ErrorName error_ErrorMessage error_ErrorDetails)))