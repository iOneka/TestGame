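; BP_Gun is the holdable firearm logic for hitscan shooting, recoil and reloading from the owner's inventory.
; ApplyDamage and its multi-pellet shotgun variant trace from camera, then from Trigger, with spread scaled by aiming and movement speed.
; Hits deal point damage, doubled for head or neck, and client branches broadcast crosshair hit markers.
; Shooters play effects locally, while server multicasts show tracers, sounds and impacts to others.
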(event `SERVER ChangeIsFirstFire`
  (params (IsFirstFire :type Boolean))
  (set `self.Is Not First Fire` IsFirstFire))

(event `SERVER Reload Ammo`
  (params (`ID Ammunition` :type Name))
  (bind (_success _amount_to_reload) (`self.ReloadAmmo` `ID Ammunition`))
  (set `self.CurrentAmmo` _amount_to_reload))

(event `Recoil`
  (params (RecoilAmpDef :type "Float (double-precision)") (SidewaysDef :type "Float (double-precision)") (MinRandom :type "Float (double-precision)") (MaxRandom :type "Float (double-precision)") (BaseLookUpRate :type "Float (double-precision)") (BaseTurnRate :type "Float (double-precision)"))
  (bind (_direction _recoilfloat) (`Timeline|Timeline` :!via `PlayFromStart`)
    (:`Update`
      (bind _returnvalue (* (* _recoilfloat RecoilAmpDef) (`KismetMathLibrary.RandomFloatInRange` MinRandom MaxRandom)))
      (`Pawn.AddControllerPitchInput` (`self.Owner as Survival Character`) (* _returnvalue BaseLookUpRate (`GameplayStatics.GetWorldDeltaSeconds`)))
      (`Pawn.AddControllerYawInput` (`self.Owner as Survival Character`) (* (* (* SidewaysDef _returnvalue) (`KismetMathLibrary.RandomFloatInRange` -2.0 2.0)) BaseTurnRate (`GameplayStatics.GetWorldDeltaSeconds`))))))

(event `MULTICAST Effects`
  (params (Hit :type "HitResult Structure (by ref)") (`L Bullet Hit` :type Boolean) (`End Position` :type "Vector Structure"))
  (`/Game/Somewhere/Core/Libraries/BML_BP_Somewhere.Switch Has Authority 2`
    (:`Standalone`
      _)
    (:`Client`
      _))
  (`/Engine/EditorBlueprintResources/StandardMacros.IsValid` (`Pawn.GetController` (cast `Pawn` (`self.GetOwner`) :!pure true))
    (:`Is Not Valid`
      (bind (_surface_hit _water_hit_location) (`self.Hit Direction` Hit))
      (`self.Do Custom Shot Effects` _surface_hit _water_hit_location `L Bullet Hit` `End Position`))))

(event `SERVER Effects`
  (params (Hit :type "HitResult Structure (by ref)") (`L Bullet Hit` :type Boolean))
  (`self.MULTICAST Effects` Hit `L Bullet Hit`))

(fn `Apply Damage Shotguns`
  (params (Distance :type "Float (double-precision)") (ShellAmount :type Integer) (Damage :type "Float (double-precision)") (SpreadAim :type "Float (double-precision)") (SpreadWithoutAim :type "Float (double-precision)"))
  (locals (Spread :type "Float (double-precision)" :default 300.0) (`L Hit Actor` :type "Actor Object Reference") (`L Damaged Actors` :type "Array of Actor Object Reference") (Hits :type "Array of HitResult Structure") (`L Out Hit Second` :type "HitResult Structure") (`L Second Hit` :type Boolean) (`L Out Hit First` :type "HitResult Structure") (`L First End Pos` :type "Vector Structure"))
  (bind _spread (`local.Spread`))
  (bind _damage (`local.Damage`))
  (bind _l_out_hit_second (`local.L Out Hit Second`))
  (bind (_l_out_hit_second_bblockinghit _l_out_hit_second_binitialoverlap _l_out_hit_second_time _l_out_hit_second_distance _l_out_hit_second_location _l_out_hit_second_impactpoint _l_out_hit_second_normal _l_out_hit_second_impactnormal _l_out_hit_second_physmat _l_out_hit_second_hitactor) (`GameplayStatics.BreakHitResult` (`local.L Out Hit Second`)))
  (bind _l_out_hit_second_2 (`local.L Out Hit Second`))
  (bind (_bblockinghit _binitialoverlap _time _distance _location _impactpoint _normal _impactnormal _physmat _hitactor _hitcomponent _hitbonename _bonename _hititem _elementindex _faceindex _tracestart) (`GameplayStatics.BreakHitResult` _l_out_hit_second))
  (bind _returnvalue (`SceneComponent.K2_GetComponentLocation` (`self.Trigger`)))
  (bind (_location_2 _rotation) (`Controller.GetPlayerViewPoint` (`self.Owner As Player Controller`)))
  (bind _returnvalue_2 (`SceneComponent.K2_GetComponentLocation` (`self.Trigger`)))
  (bind (_bblockinghit_2 _binitialoverlap_2 _time_2 _distance_2 _location_3 _impactpoint_2 _normal_2 _impactnormal_2 _physmat_2 _hitactor_2 _hitcomponent_2 _hitbonename_2 _bonename_2 _hititem_2 _elementindex_2 _faceindex_2 _tracestart_2 _traceend) (`GameplayStatics.BreakHitResult` _l_out_hit_second_2))
  (bind _returnvalue_3 (or (== _hitbonename "Head") (== _hitbonename "neck_01")))
  (for _ (range ShellAmount)
    ;[0 0 0] Разброс
    (if (`GameplayTagAssetInterface.HasMatchingGameplayTag` (`SomewhereCharacter.AbilitySystemComponent` (`self.Owner as Survival Character`)) (struct :`TagName` "GameplayAbility.Weapon.Aim.Active"))
      (set `local.Spread` (`local.SpreadAim`))
      (else
        (set `local.Spread` (`local.SpreadWithoutAim`))))
    (set `local.Spread` (+ (* _spread (/ (`self.ShotVelocity`) 8.0)) _spread))
    ;[0 0 0] LineTrace до прицела
    (bind _output_get (set `local.L First End Pos` (+ _location_2 (* (`KismetMathLibrary.Conv_RotatorToVector` _rotation) (`local.Distance`)))))
    (bind (_outhit _returnvalue_4) (`KismetSystemLibrary.LineTraceSingle` _location_2 _output_get "TraceTypeQuery1" false (`|MakeArray` (`self.Owner as Character`) :!type "Actor Object Reference") "None" true (struct :`G` 1.0 :`B` 0.962814 :`A` 1.0) (struct :`R` 0.985269 :`G` 0.988951 :`B` 1.0 :`A` 1.0) 10.0))
    (set `local.L Out Hit First` _outhit)
    (bind _output_get_2 (set `self.Bullet Hit` _returnvalue_4))
    (if _output_get_2
      ;[0 0 0] Выстрел в объект
      (bind (_outhit_2 _returnvalue_5) (`KismetSystemLibrary.LineTraceSingle` _returnvalue (+ (* (+ (`KismetMathLibrary.GetForwardVector` (`KismetMathLibrary.FindLookAtRotation` _returnvalue (`.ImpactPoint` (`GameplayStatics.BreakHitResult` (`local.L Out Hit First`))))) (`KismetMathLibrary.MakeVector` (* (`local.Spread`) (`KismetMathLibrary.RandomFloatInRange` -0.01 0.01)) (* (`local.Spread`) (`KismetMathLibrary.RandomFloatInRange` -0.01 0.01)) (* (`local.Spread`) (`KismetMathLibrary.RandomFloatInRange` -0.01 0.01)))) (`local.Distance`)) _returnvalue) "TraceTypeQuery1" false (`|MakeArray` (`self.Owner as Character`) :!type "Actor Object Reference") "None" true (struct :`R` 1.0 :`B` 0.730776 :`A` 1.0)))
      (set `local.L Out Hit Second` _outhit_2)
      (set `local.L Second Hit` _returnvalue_5)
      (else
        ;[0 0 0] Выстрел в воздух
        (bind (_outhit_3 _returnvalue_6) (`KismetSystemLibrary.LineTraceSingle` :`Start` _returnvalue_2 :`End` (+ (* (+ (`KismetMathLibrary.GetForwardVector` (`KismetMathLibrary.FindLookAtRotation` _returnvalue_2 (`local.L First End Pos`))) (`KismetMathLibrary.MakeVector` (* (`local.Spread`) (`KismetMathLibrary.RandomFloatInRange` -0.01 0.01)) (* (`local.Spread`) (`KismetMathLibrary.RandomFloatInRange` -0.01 0.01)) (* (`local.Spread`) (`KismetMathLibrary.RandomFloatInRange` -0.01 0.01)))) (`local.Distance`)) _returnvalue_2) :`TraceChannel` "TraceTypeQuery1" :`TraceColor` (struct :`R` 0.358979 :`G` 1.0 :`A` 1.0) :`TraceHitColor` (struct :`R` 0.99765 :`G` 1.0 :`A` 1.0)))
        (set `local.L Out Hit Second` _outhit_3)
        (set `local.L Second Hit` _returnvalue_6)))
    ;[0 0 0] В итоге попали или нет с учетом разброса
    (if (`local.L Second Hit`)
      ;[0 0 0] Попали
      (`/Game/Somewhere/Core/Libraries/BML_BP_Somewhere.Switch Has Authority 2`
        (:`Server`
          (`self.MULTICAST Effects` (`local.L Out Hit Second`) (`local.L Second Hit`)))
        (:`Standalone`
          (bind (_surface_hit _water_hit_location) (`self.Hit Direction` (`local.L Out Hit Second`) :!label _label))
          (`self.Do Custom Shot Effects` _surface_hit _water_hit_location (`local.L Second Hit`)))
        (:`Client`
          (goto _label)))
      (`/Game/Somewhere/Core/Libraries/BML_BP_Somewhere.Switch Has Authority 2`
        (:`Server`
          ;[0 0 0] Apply Damage
          (bind _output_get_3 (set `local.L Hit Actor` _hitactor :!label _label_2))
          (`GameplayStatics.ApplyPointDamage` _output_get_3 (`KismetMathLibrary.SelectFloat` (* _damage 2.0) _damage _returnvalue_3) _tracestart _l_out_hit_second (`self.Owner As Player Controller`) (`self.Owner as Character`) "/Game/Somewhere/Core/DamageTypes/DT_Bullet.DT_Bullet_C"))
        (:`Standalone`
          (goto _label_2))
        (:`Client`
          (cast `Pawn` _l_out_hit_second_hitactor)
          (`GameplayMessageSubsystem.K2_BroadcastMessage` (subsystem `GameplayMessageSubsystem`) (struct :`TagName` "GameplayMessage.CrosshireHit") (make `/Game/Somewhere/Objects/Items/Weapons/S_CrosshireObstacle` _returnvalue_3))))
      (else
        ;[0 0 0] Не попали из за разброса
        (`/Game/Somewhere/Core/Libraries/BML_BP_Somewhere.Switch Has Authority 2`
          (:`Server`
            (`self.MULTICAST Effects` (`local.L Out Hit Second`) (`local.L Second Hit`) _traceend))
          (:`Standalone`
            (bind (_surface_hit_2 _water_hit_location_2) (`self.Hit Direction` _l_out_hit_second_2 :!label _label_3))
            (`self.Do Custom Shot Effects` _surface_hit_2 _water_hit_location_2 (`local.L Second Hit`) _traceend))
          (:`Client`
            (goto _label_3)))))))

(fn `ApplyDamage`
  (params (SpreadAim :type "Float (double-precision)") (SpreadWithoutAim :type "Float (double-precision)") (Distance :type "Float (double-precision)") (Damage :type "Float (double-precision)") (IsNotFirstFire :type Boolean))
  (locals (`L Hit Actor` :type "Actor Object Reference") (Spread :type "Float (double-precision)" :default 0.0) (`L Out Hit First` :type "HitResult Structure") (`L First End Pos` :type "Vector Structure") (`L Out Hit Second` :type "HitResult Structure") (`L Second Hit` :type Boolean :default false))
  (bind _spread (`local.Spread`))
  (bind _damage (`local.Damage`))
  (bind _l_out_hit_second (`local.L Out Hit Second`))
  (bind _l_out_hit_second_2 (`local.L Out Hit Second`))
  (bind (_l_out_hit_second_bblockinghit _l_out_hit_second_binitialoverlap _l_out_hit_second_time _l_out_hit_second_distance _l_out_hit_second_location _l_out_hit_second_impactpoint _l_out_hit_second_normal _l_out_hit_second_impactnormal _l_out_hit_second_physmat _l_out_hit_second_hitactor) (`GameplayStatics.BreakHitResult` (`local.L Out Hit Second`)))
  (bind (_bblockinghit _binitialoverlap _time _distance _location _impactpoint _normal _impactnormal _physmat _hitactor _hitcomponent _hitbonename _bonename _hititem _elementindex _faceindex _tracestart) (`GameplayStatics.BreakHitResult` _l_out_hit_second))
  (bind _returnvalue (`SceneComponent.K2_GetComponentLocation` (`self.Trigger`)))
  (bind (_bblockinghit_2 _binitialoverlap_2 _time_2 _distance_2 _location_2 _impactpoint_2 _normal_2 _impactnormal_2 _physmat_2 _hitactor_2 _hitcomponent_2 _hitbonename_2 _bonename_2 _hititem_2 _elementindex_2 _faceindex_2 _tracestart_2 _traceend) (`GameplayStatics.BreakHitResult` _l_out_hit_second_2))
  (bind (_location_3 _rotation) (`Controller.GetPlayerViewPoint` (`self.Owner As Player Controller`)))
  (bind _returnvalue_2 (`SceneComponent.K2_GetComponentLocation` (`self.Trigger`)))
  (bind _returnvalue_3 (or (== _hitbonename "Head") (== _hitbonename "neck_01")))
  ;[0 0 0] Первый выстрел без разброса
  (if IsNotFirstFire
    ;[0 0 0] Разброс
    (if (`GameplayTagAssetInterface.HasMatchingGameplayTag` (`SomewhereCharacter.AbilitySystemComponent` (`self.Owner as Survival Character`)) (struct :`TagName` "GameplayAbility.Weapon.Aim.Active"))
      (set `local.Spread` (`local.SpreadAim`))
      (else
        (set `local.Spread` (`local.SpreadWithoutAim`))))
    (else
      (set `local.Spread` (/ (`local.SpreadAim`) 2.0))))
  (set `local.Spread` (+ (* _spread (`self.ShotVelocity`)) _spread))
  ;[0 0 0] LineTrace до прицела
  (bind _output_get (set `local.L First End Pos` (+ _location_3 (* (`KismetMathLibrary.Conv_RotatorToVector` _rotation) (`local.Distance`)))))
  (bind (_outhit _returnvalue_4) (`KismetSystemLibrary.LineTraceSingle` _location_3 _output_get "TraceTypeQuery1" false (`|MakeArray` (`self.Owner as Character`) :!type "Actor Object Reference") "None" true (struct :`G` 1.0 :`B` 0.962814 :`A` 1.0) (struct :`R` 0.985269 :`G` 0.988951 :`B` 1.0 :`A` 1.0) 10.0))
  (set `local.L Out Hit First` _outhit)
  (bind _output_get_2 (set `self.Bullet Hit` _returnvalue_4))
  (if _output_get_2
    ;[0 0 0] Выстрел в объект
    (bind (_outhit_2 _returnvalue_5) (`KismetSystemLibrary.LineTraceSingle` _returnvalue (+ (* (+ (`KismetMathLibrary.GetForwardVector` (`KismetMathLibrary.FindLookAtRotation` _returnvalue (`.ImpactPoint` (`GameplayStatics.BreakHitResult` (`local.L Out Hit First`))))) (`KismetMathLibrary.MakeVector` (* (`local.Spread`) (`KismetMathLibrary.RandomFloatInRange` -0.01 0.01)) (* (`local.Spread`) (`KismetMathLibrary.RandomFloatInRange` -0.01 0.01)) (* (`local.Spread`) (`KismetMathLibrary.RandomFloatInRange` -0.01 0.01)))) (`local.Distance`)) _returnvalue) "TraceTypeQuery1" false (`|MakeArray` (`self.Owner as Character`) :!type "Actor Object Reference") "None" true (struct :`R` 1.0 :`B` 0.730776 :`A` 1.0)))
    (set `local.L Out Hit Second` _outhit_2)
    (set `local.L Second Hit` _returnvalue_5)
    (else
      ;[0 0 0] Выстрел в воздух
      (bind (_outhit_3 _returnvalue_6) (`KismetSystemLibrary.LineTraceSingle` _returnvalue_2 (+ (* (+ (`KismetMathLibrary.GetForwardVector` (`KismetMathLibrary.FindLookAtRotation` _returnvalue_2 (`local.L First End Pos`))) (`KismetMathLibrary.MakeVector` (* (`local.Spread`) (`KismetMathLibrary.RandomFloatInRange` -0.01 0.01)) (* (`local.Spread`) (`KismetMathLibrary.RandomFloatInRange` -0.01 0.01)) (* (`local.Spread`) (`KismetMathLibrary.RandomFloatInRange` -0.01 0.01)))) (`local.Distance`)) _returnvalue_2) "TraceTypeQuery1" false (`|MakeArray` (`self.Owner as Character`) :!type "Actor Object Reference") "None" true (struct :`R` 0.358979 :`G` 1.0 :`A` 1.0) (struct :`R` 0.99765 :`G` 1.0 :`A` 1.0)))
      (set `local.L Out Hit Second` _outhit_3)
      (set `local.L Second Hit` _returnvalue_6)))
  ;[0 0 0] В итоге попали или нет с учетом разброса
  (if (`local.L Second Hit`)
    ;[0 0 0] Попали
    (`/Game/Somewhere/Core/Libraries/BML_BP_Somewhere.Switch Has Authority 2`
      (:`Server`
        (`self.MULTICAST Effects` (`local.L Out Hit Second`) (`local.L Second Hit`)))
      (:`Standalone`
        (bind (_surface_hit _water_hit_location) (`self.Hit Direction` (`local.L Out Hit Second`) :!label _label))
        (`self.Do Custom Shot Effects` _surface_hit _water_hit_location (`local.L Second Hit`)))
      (:`Client`
        (goto _label)))
    (`/Game/Somewhere/Core/Libraries/BML_BP_Somewhere.Switch Has Authority 3`
      (:`Server`
        ;[0 0 0] Apply Damage
        (bind _output_get_3 (set `local.L Hit Actor` _hitactor :!label _label_2))
        (`GameplayStatics.ApplyPointDamage` _output_get_3 (`KismetMathLibrary.SelectFloat` (* _damage 2.0) _damage _returnvalue_3) _tracestart _l_out_hit_second (`self.Owner As Player Controller`) (`self.Owner as Character`) "/Game/Somewhere/Core/DamageTypes/DT_Bullet.DT_Bullet_C"))
      (:`Standalone (Server)`
        (goto _label_2))
      (:`Standalone (Cient)`
        (cast `Pawn` _l_out_hit_second_hitactor :!label _label_3)
        (`GameplayMessageSubsystem.K2_BroadcastMessage` (subsystem `GameplayMessageSubsystem`) (struct :`TagName` "GameplayMessage.CrosshireHit") (make `/Game/Somewhere/Objects/Items/Weapons/S_CrosshireObstacle` _returnvalue_3)))
      (:`Client`
        (goto _label_3)))
    (else
      ;[0 0 0] Не попали из за разброса
      (`/Game/Somewhere/Core/Libraries/BML_BP_Somewhere.Switch Has Authority 2`
        (:`Server`
          (`self.MULTICAST Effects` (`local.L Out Hit Second`) (`local.L Second Hit`) _traceend))
        (:`Standalone`
          (bind (_surface_hit_2 _water_hit_location_2) (`self.Hit Direction` _l_out_hit_second_2 :!label _label_4))
          (`self.Do Custom Shot Effects` _surface_hit_2 _water_hit_location_2 (`local.L Second Hit`) _traceend))
        (:`Client`
          (goto _label_4))))))

(fn `Do Custom Shot Effects`
  (params (Hit :type "HitResult Structure") (`Water Hit` :type "Vector Structure") (`L Bullet Hit` :type Boolean) (`End Position` :type "Vector Structure"))
  (locals (`Impact Point` :type "Vector Structure" :default (0.0 0.0 0.0)) (TraceEnd :type "Vector Structure" :default (0.0 0.0 0.0)) (`Impact Normal` :type "Vector Structure" :default (0.0 0.0 0.0)) (`Hit Component` :type "PrimitiveComponent Object Reference") (`Hit Actor` :type "Actor Object Reference"))
  (bind _water_hit (`local.Water Hit`))
  (bind (_bblockinghit _binitialoverlap _time _distance _location _impactpoint _normal _impactnormal _physmat _hitactor _hitcomponent _hitbonename _bonename _hititem _elementindex _faceindex _tracestart _traceend) (`GameplayStatics.BreakHitResult` (`local.Hit`)))
  (if `L Bullet Hit`
    (`|ExecutionSequence`
      (:`then_0`
        (set `local.Impact Point` _impactpoint)
        (set `local.TraceEnd` _traceend)
        (set `local.Hit Component` _hitcomponent)
        (set `local.Impact Normal` _impactnormal)
        (set `local.Hit Actor` _hitactor))
      (:`then_1`
        (if (`KismetMathLibrary.BooleanNOR` (`KismetMathLibrary.EqualExactly_VectorVector` _water_hit) (`KismetMathLibrary.EqualExactly_VectorVector` _water_hit (1.0 1.0 1.0)))
          (`NiagaraFunctionLibrary.SpawnSystemAtLocation` "/Game/Somewhere/Effects/Particles/Niagara/NS_WaterSplash_Small.NS_WaterSplash_Small" (`local.Water Hit`))
          (`GameplayStatics.SpawnSoundAtLocation` "/Game/Somewhere/Audio/Impact/WAV_WaterHit_01.WAV_WaterHit_01" (`local.Water Hit`) (struct) 1.0 1.0 0.0 null null)))
      (:`then_2`
        (`GameplayStatics.SpawnEmitterAttached` "/Game/Somewhere/Effects/Particles/P_TriggerFire.P_TriggerFire" (`self.Trigger`))
        (bind _returnvalue (`NiagaraFunctionLibrary.SpawnSystemAtLocation` "/Game/Somewhere/Effects/Particles/Niagara/NS_BulletTrace.NS_BulletTrace" (`SceneComponent.K2_GetComponentLocation` (`self.Trigger`)) (struct) (4.0 4.0 4.0) true false))
        (`FXSystemComponent.SetVectorParameter` _returnvalue "End Location" (select `bool` (`local.L Bullet Hit`) :`false` (`local.Impact Point`) :`true` (`local.TraceEnd`)))
        (`ActorComponent.Activate` _returnvalue true)
        (bind _asbp_weapon_base (cast `/Game/Somewhere/Objects/Items/Weapons/BP_WeaponBase` (`/Game/Somewhere/Core/Player/Inventory/BPC_InventoryComponent.Current Holdable` (`/Game/Somewhere/Core/Player/CH_SurvivalCharacter.BPC_InventoryComponent` (`self.Owner as Survival Character`)))))
        (`GameplayStatics.PlaySoundAtLocation` (`/Game/Somewhere/Objects/Items/Weapons/BP_WeaponBase.FireSound` _asbp_weapon_base) (`SceneComponent.K2_GetComponentLocation` (`Character.Mesh` (`self.Owner as Survival Character`))) (struct) 1.0 1.0 0.0 null null null null)
        (if (`local.L Bullet Hit`)
          (bind _asch_survival_character (cast `/Game/Somewhere/Core/Player/CH_SurvivalCharacter` (`local.Hit Actor`))
            (:`then`
              (if (not (`KismetArrayLibrary.Array_Contains` (`ActorComponent.ComponentTags` (`Character.Mesh` _asch_survival_character)) "Vehicle"))
                (`NiagaraFunctionLibrary.SpawnSystemAtLocation` "/Game/Somewhere/Effects/Particles/Niagara/NS_BloodSplash.NS_BloodSplash" (`local.Impact Point`))))
            (:`CastFailed`
              (bind _returnvalue_2 (`GameplayStatics.SpawnDecalAttached` "/Game/Somewhere/MaterialLibrary/Material/M_BulletHole.M_BulletHole" (2.0 2.0 2.0) (`local.Hit Component`) "None" (`local.Impact Point`) (`KismetMathLibrary.Conv_VectorToRotator` (`local.Impact Normal`)) "KeepWorldPosition" 30.0))
              (`/Engine/EditorBlueprintResources/StandardMacros.IsValid` _returnvalue_2
                (:`Is Valid`
                  (`DecalComponent.SetFadeOut` _returnvalue_2 25.0 1.0 false)
                  (`DecalComponent.SetFadeScreenSize` _returnvalue_2 0.0015))
                (:`Is Not Valid`
                  _))
              (if (`KismetMathLibrary.EqualExactly_VectorVector` (`local.Water Hit`))
                (`GameplayStatics.SpawnEmitterAtLocation` "/Game/Somewhere/Effects/Particles/P_ImpactSmoke.P_ImpactSmoke" (`local.Impact Point`))
                (`GameplayStatics.SpawnSoundAtLocation` "/Game/Somewhere/Audio/Impact/CUE_BulletImpact.CUE_BulletImpact" (`local.Impact Point`) (struct) 1.0 1.0 0.0 "/Game/Somewhere/Audio/Attenuation/SA_Footsteps.SA_Footsteps" null)))))))
    (else
      (`GameplayStatics.SpawnEmitterAttached` "/Game/Somewhere/Effects/Particles/P_TriggerFire.P_TriggerFire" (`self.Trigger`))
      (bind _returnvalue_3 (`NiagaraFunctionLibrary.SpawnSystemAtLocation` "/Game/Somewhere/Effects/Particles/Niagara/NS_BulletTrace.NS_BulletTrace" (`SceneComponent.K2_GetComponentLocation` (`self.Trigger`)) (struct) (4.0 4.0 4.0) true false))
      (`FXSystemComponent.SetVectorParameter` _returnvalue_3 "End Location" (`local.End Position`))
      (`ActorComponent.Activate` _returnvalue_3 true)
      (bind _asbp_weapon_base_2 (cast `/Game/Somewhere/Objects/Items/Weapons/BP_WeaponBase` (`/Game/Somewhere/Core/Player/Inventory/BPC_InventoryComponent.Current Holdable` (`/Game/Somewhere/Core/Player/CH_SurvivalCharacter.BPC_InventoryComponent` (`self.Owner as Survival Character`)))))
      (`GameplayStatics.PlaySoundAtLocation` (`/Game/Somewhere/Objects/Items/Weapons/BP_WeaponBase.FireSound` _asbp_weapon_base_2) (`SceneComponent.K2_GetComponentLocation` (`Character.Mesh` (`self.Owner as Survival Character`))) (struct) 1.0 1.0 0.0 null null null null))))

(fn `Hit Direction`
  (params (Hit :type "HitResult Structure (by ref)"))
  (returns (`Surface Hit` :type "HitResult Structure") (`Water Hit Location` :type "Vector Structure"))
  (locals (`Water Hit L` :type "Vector Structure"))
  (bind (_bblockinghit _binitialoverlap _time _distance _location _impactpoint _normal _impactnormal _physmat _hitactor) (`GameplayStatics.BreakHitResult` Hit))
  (if (not _bblockinghit)
    (cast `/Game/Somewhere/Core/BP_Water` _hitactor)
    (set `local.Water Hit L` (select `bool` (> _distance 0.0) :`false` (1.0 1.0 1.0) :`true` _impactpoint)))
  (return Hit (`local.Water Hit L`)))

(fn `OnRep_Bullet Hit`)

(fn `ReloadAmmo`
  (params (`ID Ammunition` :type Name))
  (returns (Success :type Boolean) (`Amount to Reload` :type Integer))
  (locals (`L Requied Ammo` :type Integer) (`L Cached Indexes` :type "Array of Integer") (`L Reloaded Amount` :type Integer) (`L Actual Reloaded Amount` :type Integer) (`L Modified Requied Ammo` :type Integer))
  (bind _l_modified_requied_ammo (`local.L Modified Requied Ammo`))
  (bind _main_container (`/Game/Somewhere/Core/Player/Inventory/BPC_InventoryComponent.Main Container` (`/Game/Somewhere/Core/Player/CH_SurvivalCharacter.BPC_InventoryComponent` (`self.Owner as Survival Character`))))
  (set `local.L Requied Ammo` (- (`self.AmmoMagazinSize`) (`self.CurrentAmmo`)))
  (bind _output_get (set `local.L Cached Indexes` (`ItemContainer.FindAllCellsWithItem` _main_container `ID Ammunition`)))
  (for _array_element _output_get
    (bind _output_get_2 (set `local.L Modified Requied Ammo` (- (`local.L Requied Ammo`) (`local.L Reloaded Amount`))))
    (if (> _output_get_2 0)
      (bind (_id _amount) (break `InventoryItem` (`ItemContainer.GetCell` _main_container _array_element)))
      (if (> _amount _l_modified_requied_ammo)
        (bind _output_get_3 (set `local.L Actual Reloaded Amount` _l_modified_requied_ammo))
        (`ItemContainer.RemoveItemAmountFromCell` _main_container _array_element _output_get_3)
        (set `local.L Reloaded Amount` (+ _l_modified_requied_ammo (`local.L Reloaded Amount`)))
        (else
          (bind _output_get_4 (set `local.L Actual Reloaded Amount` _amount))
          (`ItemContainer.RemoveItemAmountFromCell` _main_container _array_element _output_get_4)
          (set `local.L Reloaded Amount` (+ (`local.L Reloaded Amount`) (`local.L Actual Reloaded Amount`)))))
      (else
        (break))))
  (if (> (`local.L Reloaded Amount`) 0)
    (return true (- (`self.AmmoMagazinSize`) (- (`local.L Requied Ammo`) (`local.L Reloaded Amount`))))
    (else
      (return false 0))))

(fn `ShotVelocity`
  (returns (ReturnValue :type "Float (double-precision)"))
  (return (`KismetMathLibrary.FClamp` (/ (`KismetMathLibrary.VSize` (`self.GetVelocity` (`self.Owner as Survival Character`))) 1000.0))))

(fn `UserConstructionScript`
  (`parent.UserConstructionScript`))