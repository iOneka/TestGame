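; Survival game mode that keeps logged-out players' characters in the world as sleeping bodies.
; PreLogout stores the character in a map keyed by PlayFab ID, puts it to sleep and unpossesses it.
; StartPlayer repossesses and wakes that body, or spawns a new survival character at a random PlayerStart.
; It also logs the server into PlayFab with a custom ID and spawns a voice chat actor on each PostLogin.
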(event `self.K2_PostLogin`
  (params (NewPlayer :type "PlayerController Object Reference"))
  (`|SpawnActorFromClass` "/Script/UniversalVoiceChatPro.PlayerVoiceChatActor" (`KismetMathLibrary.MakeTransform` (0.0 0.0 0.0)) "AlwaysSpawn" "MultiplyWithRoot" NewPlayer (`KismetMathLibrary.RandomInteger` 10000) "/Somewhere/AlwaysCook/VoiceAttenuation.uasset" false true true 1000.0 null))

(event `self.ReceiveBeginPlay`
  (`PlayFabClientAPI.LoginWithCustomID` (make `ClientLoginWithCustomIDRequest` true "DEDICATED_SERVER") (delegate `SuccessLoginServer`) (delegate `FailedLoginServer`)))

(event `self.K2_PreLogout`
  (params (ExitingController :type "PlayerController Object Reference"))
  (`self.Handle Pre Logout` ExitingController))

(event `SuccessLoginServer`
  (params (result :type "ClientLoginResult Structure") (customData :type "Object Object Reference")))

(event `FailedLoginServer`
  (params (error :type "PlayFabError Structure") (customData :type "Object Object Reference")))

(event `self.K2_OnLogout`
  (params (ExitingController :type "Controller Object Reference")))

(event `self.StartPlayer`
  (params (NewPlayer :type "SomewherePlayerController Object Reference"))
  (`self.Handle Start Player` NewPlayer))

(event `self.K2_RestartPlayer`
  (params (NewPlayer :type "PlayerController Object Reference"))
  (`self.Handle Restart Player` NewPlayer))

(fn `Get First Player Start`
  (returns (`Player Start` :type "PlayerStart Object Reference") (Transform :type "Transform Structure (by ref)"))
  (bind _outactors (`GameplayStatics.GetAllActorsOfClass` "/Script/Engine.PlayerStart"))
  (bind _output (`|GetArrayItem` _outactors))
  (return _output (`self.GetTransform` _output)))

(fn `Get Random Player Start`
  (returns (`Player Start` :type "PlayerStart Object Reference") (Transform :type "Transform Structure (by ref)"))
  (bind _outactors (`GameplayStatics.GetAllActorsOfClass` "/Script/Engine.PlayerStart"))
  (bind _outitem (`KismetArrayLibrary.Array_Random` _outactors))
  (return _outitem (`self.GetTransform` _outitem)))

(fn `Handle Pre Logout`
  (params (Controller :type "Controller Object Reference"))
  (locals (`L Somewhere Character` :type "SomewhereCharacter Object Reference") (`L Somewhere Player Controller` :type "SomewherePlayerController Object Reference") (`L PlayFab ID` :type String))
  ;[0 0 0] Comment
  (bind _output_get (set `local.L Somewhere Player Controller` (cast `SomewherePlayerController` Controller :!pure true)))
  (set `local.L PlayFab ID` (`SomewherePlayerState.PlayFabID` (`SomewherePlayerController.GetSomewherePlayerState` _output_get)))
  (set `local.L Somewhere Character` (`SomewherePlayerController.GetLinkedSomewhereCharacter` (`local.L Somewhere Player Controller`)))
  (`KismetSystemLibrary.PrintText` (`|FormatText` "PRELOGOUT \n \nController - {pc} \nCharacter - {ch} \nPlayFabID - {pfid}" (`local.L Somewhere Player Controller`) (`local.L Somewhere Character`) (`local.L PlayFab ID`)))
  ;[0 0 0] Добавляем тело в список спящих
  (`BlueprintMapLibrary.Map_Add` (`self.SleepingBodies`) (`local.L PlayFab ID`) (`local.L Somewhere Character`))
  (bind _keys (`BlueprintMapLibrary.Map_Keys` (`self.SleepingBodies`)))
  (for _array_element _keys
    (`KismetSystemLibrary.PrintText` (`|FormatText` "Key: {k} VALUE: {v}" _array_element (`BlueprintMapLibrary.Map_Find` (`self.SleepingBodies`) _array_element))))
  (`SomewhereCharacter.SetSleepingState` (`local.L Somewhere Character`) true)
  (`Controller.UnPossess` (`local.L Somewhere Player Controller`)))

(fn `Handle Restart Player`
  (params (`Player Controller` :type "PlayerController Object Reference"))
  (`Controller.UnPossess` `Player Controller`)
  (bind _returnvalue (`|SpawnActorFromClass` "/Game/Somewhere/Core/Player/CH_SurvivalCharacter.CH_SurvivalCharacter_C" (`.Transform` (`self.Get Random Player Start`)) "AdjustIfPossibleButAlwaysSpawn" "MultiplyWithRoot" null false false false false false null))
  (`Controller.Possess` (`local.Player Controller`) _returnvalue))

(fn `Handle Start Player`
  (params (`Player Controller` :type "PlayerController Object Reference"))
  (locals (`L Somewhere Player Controller` :type "SomewherePlayerController Object Reference") (`L Somewhere Player State` :type "SomewherePlayerState Object Reference") (`L PlayFab ID` :type String) (`L Somewhere Character` :type "SomewhereCharacter Object Reference"))
  (bind (_value _returnvalue) (`BlueprintMapLibrary.Map_Find` (`self.SleepingBodies`) (`local.L PlayFab ID`)))
  ;[0 0 0] Comment
  (bind _assomewhere_player_controller (cast `SomewherePlayerController` `Player Controller`))
  (bind _output_get (set `local.L Somewhere Player Controller` _assomewhere_player_controller))
  (bind _output_get_2 (set `local.L Somewhere Player State` (`SomewherePlayerController.GetSomewherePlayerState` _output_get)))
  (set `local.L PlayFab ID` (`SomewherePlayerState.PlayFabID` _output_get_2))
  ;[0 0 0] Есть ли спящее тело игрока на карте?
  (if (and (`KismetSystemLibrary.IsValid` _value) _returnvalue)
    ;[0 0 0] Вселяемся в тело
    (bind _output_get_3 (set `local.L Somewhere Character` (`BlueprintMapLibrary.Map_Find` (`self.SleepingBodies`) (`local.L PlayFab ID`))))
    (`Controller.Possess` (`local.L Somewhere Player Controller`) _output_get_3)
    (`SomewhereCharacter.SetSleepingState` (`local.L Somewhere Character`) false)
    (else
      ;[0 0 0] Спавним новое тело
      (`self.RestartPlayer` (`local.L Somewhere Player Controller`)))))

(fn `UserConstructionScript`)