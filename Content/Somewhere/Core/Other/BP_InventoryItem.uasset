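; World pickup actor for an inventory item, showing the mesh, label, amount and icon from its item definition.
; Construction previews the mesh and clamps stack size, while BeginPlay loads it asynchronously and OnRep refreshes prompt data for replicated items.
; An interaction volume adds or removes a HUD prompt on standalone and client only.
; Pressing it calls the player's inventory component, which sends a server pickup if the local check passes.
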(event `self.BPC_InteractiveByVolume.On Player Entered Interactive Volume`
  (params (Character :type "Character Object Reference"))
  (`/Game/Somewhere/Core/Libraries/BML_BP_Somewhere.Switch Has Authority 2`
    (:`Standalone`
      _)
    (:`Client`
      _))
  (bind _returnvalue (`InteractionWidget.AddPrompt` (`HUDWidget.InteractionWidget` (`SomewhereStatics.GetHUDWidget`)) (`self.Prompt Icon`) (`self.Prompt Text`)))
  (bind _output_get (set `self.Current Prompt` _returnvalue))
  (add `InteractionPrompt.OnPromptPressed` _output_get (`|CreateDelegate` :!event `Event On Interaction Prompt Pressed`)))

(event `self.ReceiveBeginPlay`
  (`|ExecutionSequence`
    (:`then_0`
      ;[0 0 0] Item Definition
      (set `self.Item Definition` (`InventoryStatics.GetItemDefinitionFromItem` (`self.Inventory Item`))))
    (:`then_1`
      ;[0 0 0] Mesh
      (bind _object (`|LoadAsset` (`.Mesh` (break `ItemDefinition` (`self.Item Definition`))))
        (:`Completed`
          (bind _asstatic_mesh (cast `StaticMesh` _object))
          (`StaticMeshComponent.SetStaticMesh` (`self.Item Mesh`) _asstatic_mesh)
          (if (`KismetSystemLibrary.IsStandalone`)
            (`ActorComponent.Activate` (`self.BPC_InteractiveByVolume`) false)
            (elif (not (`KismetTextLibrary.TextIsEmpty` (`self.Prompt Text`)))
              (`ActorComponent.Activate` (`self.BPC_InteractiveByVolume`) false))))))
    (:`then_2`
      ;[0 0 0] Prompt Text
      (if (<= (`.Amount` (break `InventoryItem` (`self.Inventory Item`))) 1)
        (set `self.Prompt Text` (`.Label` (break `ItemDefinition` (`self.Item Definition`))))
        (else
          (set `self.Prompt Text` (`|FormatText` "{name} x{amount}" (`.Label` (break `ItemDefinition` (`self.Item Definition`))) (`.Amount` (break `InventoryItem` (`self.Inventory Item`)))))))
      ;[0 0 0] Prompt Icon
      (set `self.Prompt Icon` (`.Icon` (break `ItemDefinition` (`self.Item Definition`)))))))

(event `self.BPC_InteractiveByVolume.On Player Exited Interactive Volume`
  (params (Character :type "Character Object Reference"))
  (`/Game/Somewhere/Core/Libraries/BML_BP_Somewhere.Switch Has Authority 2`
    (:`Standalone`
      _)
    (:`Client`
      _))
  (`InteractionWidget.RemovePrompt` (`HUDWidget.InteractionWidget` (`SomewhereStatics.GetHUDWidget`)) (`self.Current Prompt`))
  (clear `InteractionPrompt.OnPromptPressed` (`self.Current Prompt`)))

(event `Event On Interaction Prompt Pressed`
  (bind _returnvalue (`self.GetComponentByClass` (`GameplayStatics.GetPlayerCharacter` 0) "/Game/Somewhere/Core/Player/Inventory/BPC_InventoryComponent.BPC_InventoryComponent_C"))
  (`/Engine/EditorBlueprintResources/StandardMacros.IsValid` self
    (:`Is Valid`
      (bind _success (`/Game/Somewhere/Core/Player/Inventory/BPC_InventoryComponent.Pick Up Item` _returnvalue self))
      (if _success
        (`/Game/Somewhere/Core/Player/Inventory/BPC_InventoryComponent.SERVER Pickup Item` _returnvalue self)))))

(event `CustomEvent`)

(event `self.ReceiveEndPlay`
  (params (EndPlayReason :type "EEndPlayReason Enum" :default "Destroyed"))
  (bind _returnvalue (`SomewhereStatics.GetHUDWidget`))
  (`/Game/Somewhere/Core/Libraries/BML_BP_Somewhere.Switch Has Authority 2`
    (:`Standalone`
      _)
    (:`Client`
      _))
  (bind _current_prompt (`self.Current Prompt`)
    (:`then`
      (`/Engine/EditorBlueprintResources/StandardMacros.IsValid` _returnvalue
        (:`Is Valid`
          (`InteractionWidget.RemovePrompt` (`HUDWidget.InteractionWidget` _returnvalue) _current_prompt))))
    (:`else`)))

(fn `OnRep_Inventory Item`
  (set `self.Item Definition` (`InventoryStatics.GetItemDefinitionFromItem` (`self.Inventory Item`)))
  ;[0 0 0] Prompt Text
  (if (<= (`.Amount` (break `InventoryItem` (`self.Inventory Item`))) 1)
    (set `self.Prompt Text` (`.Label` (break `ItemDefinition` (`self.Item Definition`))))
    (else
      (set `self.Prompt Text` (`|FormatText` "{name} x{amount}" (`.Label` (break `ItemDefinition` (`self.Item Definition`))) (`.Amount` (break `InventoryItem` (`self.Inventory Item`)))))))
  ;[0 0 0] Prompt Icon
  (set `self.Prompt Icon` (`.Icon` (break `ItemDefinition` (`self.Item Definition`))))
  (`ActorComponent.Activate` (`self.BPC_InteractiveByVolume`) false))

(fn `UserConstructionScript`
  (bind (_inventory_item_id _inventory_item_amount _inventory_item_cell _inventory_item_custominteger _inventory_item_durability _inventory_item_additionaldata) (break `InventoryItem` (`self.Inventory Item`)))
  (bind _inventory_item (`self.Inventory Item`))
  (bind ((`Label` _label) (`Stack` _stack)) (break `ItemDefinition` (`self.Item Definition`)))
  ;[0 0 0] Item Definition
  (if (`InventoryStatics.IsValid` _inventory_item)
    (set `self.Item Definition` (`InventoryStatics.GetItemDefinitionFromItem` _inventory_item))
    (`|ExecutionSequence`
      (:`then_0`
        ;[0 0 0] Mesh
        (bind _returnvalue (`KismetSystemLibrary.LoadAsset_Blocking` (`.Mesh` (break `ItemDefinition` (`self.Item Definition`)))))
        (bind _asstatic_mesh (cast `StaticMesh` _returnvalue))
        (`StaticMeshComponent.SetStaticMesh` (`self.Item Mesh`) _asstatic_mesh))
      (:`then_1`
        ;[0 0 0] Item Data stack Failsafe
        (if (> (`.Amount` (break `InventoryItem` (`self.Inventory Item`))) _stack)
          (set `self.Inventory Item` (make `InventoryItem` _inventory_item_id _stack _inventory_item_cell _inventory_item_custominteger _inventory_item_durability _inventory_item_additionaldata)))))))