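; Map data actor that builds the minimap and big map materials and drives optional fog of war.
; Construct Minimap creates dynamic material instances with textures, world bounds, zoom and border color, plus a render-target fog mask shared by both maps.
; A looping timer paints the player's vision into that mask by drawing a material at the pawn's normalized world position.
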(event `self.ReceiveBeginPlay`
  ;[1 1 1] Update Player Vision in Fog
  (if (`self.Enable Fog Of War`)
    (`KismetSystemLibrary.K2_SetTimer` null "Update Player Vision" (`self.Fog Of War Update Time`) true)))

(fn `Construct Minimap`
  (bind _fog_of_war_mask_resolution (`self.Fog Of War Mask Resolution`))
  (bind _world_middle_coordinations_x (`KismetMathLibrary.BreakVector2D` (`self.World Middle Coordinations`)))
  (bind (_world_middle_coordinations_x_2 _world_middle_coordinations_y) (`KismetMathLibrary.BreakVector2D` (`self.World Middle Coordinations`)))
  (bind (_world_middle_coordinations_x_3 _world_middle_coordinations_y_2) (`KismetMathLibrary.BreakVector2D` (`self.World Middle Coordinations`)))
  (bind (_world_middle_coordinations_x_4 _world_middle_coordinations_y_3) (`KismetMathLibrary.BreakVector2D` (`self.World Middle Coordinations`)))
  (bind _dynamic_minimap_material (`self.Dynamic Minimap Material`))
  (bind (_world_middle_coordinations_x_5 _world_middle_coordinations_y_4) (`KismetMathLibrary.BreakVector2D` (`self.World Middle Coordinations`)))
  (bind (_world_middle_coordinations_x_6 _world_middle_coordinations_y_5) (`KismetMathLibrary.BreakVector2D` (`self.World Middle Coordinations`)))
  (bind _dynamic_bigmap_material (`self.Dynamic Bigmap Material`))
  ;[1 1 1] Create Dynamic Material for Minimap
  (bind _returnvalue (`KismetMaterialLibrary.CreateDynamicMaterialInstance` "/Game/Somewhere/MaterialLibrary/Material/Minimap/M_Map_Base.M_Map_Base"))
  (set `self.Dynamic Minimap Material` _returnvalue)
  ;[1 1 1] Create Dynamic Material for Bigmap
  (bind _returnvalue_2 (`KismetMaterialLibrary.CreateDynamicMaterialInstance` "/Game/Somewhere/MaterialLibrary/Material/Minimap/M_Map_Base.M_Map_Base"))
  (set `self.Dynamic Bigmap Material` _returnvalue_2)
  ;[1 1 1] Set Map Texture
  (`MaterialInstanceDynamic.SetTextureParameterValue` (`self.Dynamic Minimap Material`) "MapTexture" (`self.Minimap Texture`))
  (`MaterialInstanceDynamic.SetTextureParameterValue` (`self.Dynamic Bigmap Material`) "MapTexture" (`self.BigMap Texture`))
  ;[1 1 1] Set Mask Texture
  (`MaterialInstanceDynamic.SetTextureParameterValue` (`self.Dynamic Minimap Material`) "MaskTexture" (`self.Minimap Mask Texture`))
  ;[1 1 1] BorderColor
  (`MaterialInstanceDynamic.SetVectorParameterValue` (`self.Dynamic Minimap Material`) "Border Color" (`self.Zone Color`))
  ;[1 1 1] Set World Size
  (`MaterialInstanceDynamic.SetScalarParameterValue` (`self.Dynamic Minimap Material`) "LevelSize" (`self.World Size`))
  (`MaterialInstanceDynamic.SetScalarParameterValue` (`self.Dynamic Bigmap Material`) "LevelSize" (`self.World Size`))
  ;[1 1 1] Set X Middle Location
  (`MaterialInstanceDynamic.SetScalarParameterValue` (`self.Dynamic Minimap Material`) "Minimap Middle X" _world_middle_coordinations_x)
  (`MaterialInstanceDynamic.SetScalarParameterValue` (`self.Dynamic Bigmap Material`) "Minimap Middle X" _world_middle_coordinations_x)
  ;[1 1 1] Set Y Middle Location
  (`MaterialInstanceDynamic.SetScalarParameterValue` (`self.Dynamic Minimap Material`) "Minimap Middle Y" _world_middle_coordinations_y)
  (`MaterialInstanceDynamic.SetScalarParameterValue` (`self.Dynamic Bigmap Material`) "Minimap Middle Y" _world_middle_coordinations_y)
  ;[1 1 1] Set Bigmap X Y Coordinations to middle
  (`MaterialInstanceDynamic.SetScalarParameterValue` (`self.Dynamic Bigmap Material`) "X" _world_middle_coordinations_x_4)
  (`MaterialInstanceDynamic.SetScalarParameterValue` (`self.Dynamic Bigmap Material`) "Y" _world_middle_coordinations_y_3)
  ;[1 1 1] Set Zoom Value (Big Map Default 1)
  (`MaterialInstanceDynamic.SetScalarParameterValue` (`self.Dynamic Minimap Material`) "Zoom" (`self.Minimap Zoom`))
  (`MaterialInstanceDynamic.SetScalarParameterValue` (`self.Dynamic Bigmap Material`) "Zoom" 1.0)
  ;[1 1 1] BorderColor
  (`MaterialInstanceDynamic.SetVectorParameterValue` (`self.Dynamic Bigmap Material`) "Border Color" (`self.Zone Color`))
  (if (`self.Enable Fog Of War`)
    ;[1 1 1] Create Render Target for dynamic Mask
    (bind _returnvalue_3 (`KismetRenderingLibrary.CreateRenderTarget2D` _fog_of_war_mask_resolution _fog_of_war_mask_resolution))
    (set `self.Fog Of War Mask` _returnvalue_3)
    ;[0.1101 0.4313 1] Minimap
    ;;[1 1 1] Create Fog OF War Material
    (bind _returnvalue_4 (`KismetMaterialLibrary.CreateDynamicMaterialInstance` "/Game/Somewhere/MaterialLibrary/Material/Minimap/M_FogOfWar_Mask.M_FogOfWar_Mask"))
    (bind _output_get (set `self.Minimap Fog Of War Material` _returnvalue_4))
    ;;[1 1 1] Set Fog Texture
    (`MaterialInstanceDynamic.SetTextureParameterValue` _output_get "FogTexture" (`self.Fog Of War Texture`))
    ;;[1 1 1] Set Fog Mask
    (`MaterialInstanceDynamic.SetTextureParameterValue` _output_get "FogMask" (`self.Fog Of War Mask`))
    ;;[1 1 1] Set World Size
    (`MaterialInstanceDynamic.SetScalarParameterValue` _output_get "LevelSize" (`self.World Size`))
    ;;[1 1 1] Set Middle Location
    (`MaterialInstanceDynamic.SetScalarParameterValue` _output_get "Minimap Middle X" _world_middle_coordinations_x_5)
    (`MaterialInstanceDynamic.SetScalarParameterValue` _output_get "Minimap Middle Y" _world_middle_coordinations_y_4)
    ;;[1 1 1] Zoom
    (`MaterialInstanceDynamic.SetScalarParameterValue` _output_get "Zoom" (`self.Minimap Zoom`))
    ;;[1 1 1] Set Mask Texture
    (`MaterialInstanceDynamic.SetTextureParameterValue` _output_get "MaskTexture" (`self.Minimap Mask Texture`))
    (`MaterialInstanceDynamic.SetTextureParameterValue` _dynamic_minimap_material "FogMask" (`self.Fog Of War Mask`))
    (`MaterialInstanceDynamic.SetTextureParameterValue` _dynamic_minimap_material "FogTexture" (`self.Fog Of War Texture`))
    ;[1 0.2856 0.1557] Bigmap
    ;;[1 1 1] Create Fog OF War Material
    (bind _returnvalue_5 (`KismetMaterialLibrary.CreateDynamicMaterialInstance` "/Game/Somewhere/MaterialLibrary/Material/Minimap/M_FogOfWar_Mask.M_FogOfWar_Mask"))
    (bind _output_get_2 (set `self.Bigmap Fog Of War Material` _returnvalue_5))
    ;;[1 1 1] Set Fog Texture
    (`MaterialInstanceDynamic.SetTextureParameterValue` _output_get_2 "FogTexture" (`self.Fog Of War Texture`))
    ;;[1 1 1] Set Fog Mask
    (`MaterialInstanceDynamic.SetTextureParameterValue` _output_get_2 "FogMask" (`self.Fog Of War Mask`))
    ;;[1 1 1] Set World Size
    (`MaterialInstanceDynamic.SetScalarParameterValue` _output_get_2 "LevelSize" (`self.World Size`))
    ;;[1 1 1] Set Middle Location
    (`MaterialInstanceDynamic.SetScalarParameterValue` _output_get_2 "Minimap Middle X" _world_middle_coordinations_x_6)
    (`MaterialInstanceDynamic.SetScalarParameterValue` _output_get_2 "Minimap Middle Y" _world_middle_coordinations_y_5)
    ;;[1 1 1] Zoom
    (`MaterialInstanceDynamic.SetScalarParameterValue` _output_get_2 "Zoom" 1.0)
    ;;[1 1 1] Set Location to Middle
    (`MaterialInstanceDynamic.SetScalarParameterValue` _output_get_2 "X" _world_middle_coordinations_x_3)
    (`MaterialInstanceDynamic.SetScalarParameterValue` _output_get_2 "Y" _world_middle_coordinations_y_2)
    (`MaterialInstanceDynamic.SetTextureParameterValue` _dynamic_bigmap_material "FogMask" (`self.Fog Of War Mask`))
    (`MaterialInstanceDynamic.SetTextureParameterValue` _dynamic_bigmap_material "FogTexture" (`self.Fog Of War Texture`))
    (return)))

(fn `Update Player Vision`
  (locals (`L Vision Material` :type "MaterialInstanceDynamic Object Reference"))
  (bind _returnvalue (`GameplayStatics.GetPlayerPawn` 0))
  (bind _world_size (`self.World Size`))
  (bind (_world_middle_coordinations_x _world_middle_coordinations_y) (`KismetMathLibrary.BreakVector2D` (`self.World Middle Coordinations`)))
  (bind (_returnvalue_x _returnvalue_y) (`KismetMathLibrary.BreakVector` (`self.K2_GetActorLocation` _returnvalue)))
  ;[1 1 1] Modify Material
  (`/Engine/EditorBlueprintResources/StandardMacros.IsValid` _returnvalue
    (:`Is Valid`
      (bind _returnvalue_2 (`KismetMaterialLibrary.CreateDynamicMaterialInstance` "/Game/Somewhere/MaterialLibrary/Material/Minimap/M_Player_Vision.M_Player_Vision"))
      (bind _output_get (set `local.L Vision Material` _returnvalue_2))
      (`MaterialInstanceDynamic.SetScalarParameterValue` _output_get "X" (/ (- _returnvalue_x _world_middle_coordinations_x) _world_size))
      (`MaterialInstanceDynamic.SetScalarParameterValue` _output_get "Y" (/ (- _returnvalue_y _world_middle_coordinations_y) _world_size))
      (`MaterialInstanceDynamic.SetScalarParameterValue` _output_get "Size" (* (/ 1.0 (`self.World Size`)) (`self.Vision Radius`)))
      ;[1 1 1] Apply Material to Texture
      (`KismetRenderingLibrary.DrawMaterialToRenderTarget` (`self.Fog Of War Mask`) (`local.L Vision Material`)))))

(fn `UserConstructionScript`)