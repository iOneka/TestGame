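; Gameplay ability that reloads the held survival-character weapon from inventory ammo.
; Clients play the reload montage before an OnlyServerWait net sync, while authority goes straight to that sync.
; ReloadAmmo drains matching cells to fill the magazine, returning zero if nothing loads; the result overwrites the weapon's inventory count.
; It then ends and sets walk speed by grenade-aim tag; an uncalled sphere-trace ApplyDamage function is also present.
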(event `self.K2_ActivateAbility`
  (bind _as_ch_survival_character (`self.As CH Survival Character`))
  (`|ExecutionSequence`
    (:`then_0`
      ;[0 0 0] Рефы
      (bind _ascharacter (cast `Character` (`self.GetAvatarActorFromActorInfo`)))
      (bind _output_get (set `self.Character` _ascharacter))
      (bind _asplayer_controller (cast `PlayerController` (`Pawn.GetController` _output_get)))
      (set `self.Player Controller` _asplayer_controller)
      (bind _asch_survival_character (cast `/Game/Somewhere/Core/Player/CH_SurvivalCharacter` _ascharacter))
      (set `self.As CH Survival Character` _asch_survival_character))
    (:`then_2`
      (bind _asbp_weapon_base (cast `/Game/Somewhere/Objects/Items/Weapons/BP_WeaponBase` (`/Game/Somewhere/Core/Player/Inventory/BPC_InventoryComponent.Current Holdable` (`/Game/Somewhere/Core/Player/CH_SurvivalCharacter.BPC_InventoryComponent` _as_ch_survival_character))))
      ;[0 0 0] Анимация
      (`self.K2_HasAuthority`
        (:`True`
          _)
        (:`False`
          (`AbilityTask_PlayMontageAndWait.CreatePlayMontageAndWaitProxy` "None" (`/Game/Somewhere/Objects/Items/Weapons/BP_WeaponBase.Reload Animation` _asbp_weapon_base) (`/Game/Somewhere/Objects/Items/Weapons/BP_WeaponBase.Reload Animation Rate` _asbp_weapon_base)
            (:`OnCompleted`
              _))))
      (`AbilityTask_NetworkSyncPoint.WaitNetSync` "OnlyServerWait"
        (:`OnSync`
          (bind (_success _amount_to_reload) (`self.Reload ammo` (`/Game/Somewhere/Objects/Items/Weapons/BP_WeaponBase.AmmunitionID` _asbp_weapon_base)))
          (bind (_inventory_item_id _inventory_item_amount _inventory_item_cell _inventory_item_custominteger _inventory_item_durability _inventory_item_additionaldata) (break `InventoryItem` (`/Game/Somewhere/Core/Holdable/BP_Holdable.Inventory Item` _asbp_weapon_base)))
          (bind _output_get_2 (set `/Game/Somewhere/Core/Holdable/BP_Holdable.Inventory Item` (make `InventoryItem` _inventory_item_id _inventory_item_amount _inventory_item_cell _amount_to_reload _inventory_item_durability _inventory_item_additionaldata) _asbp_weapon_base))
          (`ItemContainer.SetCell` (`/Game/Somewhere/Core/Player/Inventory/BPC_InventoryComponent.Main Container` (`/Game/Somewhere/Core/Player/CH_SurvivalCharacter.BPC_InventoryComponent` (`self.As CH Survival Character`))) (`/Game/Somewhere/Core/Holdable/BP_Holdable.Cell Item` _asbp_weapon_base) _output_get_2)
          (`self.K2_EndAbility`)
          (if (`GameplayTagAssetInterface.HasMatchingGameplayTag` (`SomewhereCharacter.AbilitySystemComponent` _as_ch_survival_character) (struct :`TagName` "GameplayAbility.Grenade.Aim.Ability"))
            (set `CharacterMovementComponent.MaxWalkSpeed` 200.0 (`Character.CharacterMovement` (`self.As CH Survival Character`)))
            (else
              (set `CharacterMovementComponent.MaxWalkSpeed` 600.0 (`Character.CharacterMovement` (`self.As CH Survival Character`))))))))))

(fn `Apply Damage`
  (locals (`L Damaged Actors` :type "Array of Actor Object Reference") (`L Hit Actor` :type "Actor Object Reference"))
  (bind _character (`self.Character`))
  (bind _returnvalue (+ (`Actor.K2_GetActorLocation` _character) (* (`Actor.GetActorForwardVector` _character) 90.0)))
  ;[0 0 0] Сфера дамага спереди
  (bind (_outhits _returnvalue_2) (`KismetSystemLibrary.SphereTraceMulti` _returnvalue _returnvalue 90.0 "TraceTypeQuery1" false (`|MakeArray` (`self.Character`) :!type "Actor Object Reference") "None" true (struct :`R` 1.0 :`A` 1.0) (struct :`G` 1.0 :`A` 1.0) 1.0))
  (if _returnvalue_2
    (for _array_element _outhits
      (set `local.L Hit Actor` (`.HitActor` (`GameplayStatics.BreakHitResult` _array_element)))
      ;[0 0 0] Дамажим всех, но только по одному разу
      (if (not (`KismetArrayLibrary.Array_Contains` (`local.L Damaged Actors`) (`local.L Hit Actor`)))
        (`KismetArrayLibrary.Array_AddUnique` (`local.L Damaged Actors`) (`local.L Hit Actor`))
        (`GameplayStatics.ApplyPointDamage` (`local.L Hit Actor`) 20.0 (`KismetMathLibrary.Normal` (- (`Actor.K2_GetActorLocation` (`local.L Hit Actor`)) (`Actor.K2_GetActorLocation` (`self.Character`)))) (`GameplayStatics.MakeHitResult` false) (`self.Player Controller`) (`self.Character`) "/Game/Somewhere/Core/DamageTypes/DT_Bullet.DT_Bullet_C")))))

(fn `Reload ammo`
  (params (`Ammo ID` :type Name))
  (returns (Success :type Boolean) (`Amount to Reload` :type Integer))
  (locals (`L Requied Ammo` :type Integer) (`L Cached Indexes` :type "Array of Integer") (`L Reloaded Amount` :type Integer) (`L Modified Requied Ammo` :type Integer) (`L Actual Reloaded Amount` :type Integer) (`Weapon Base` :type "/Game/Somewhere/Objects/Items/Weapons/BP_WeaponBase Object Reference"))
  (bind _l_modified_requied_ammo (`local.L Modified Requied Ammo`))
  (bind _main_container (`/Game/Somewhere/Core/Player/Inventory/BPC_InventoryComponent.Main Container` (`/Game/Somewhere/Core/Player/CH_SurvivalCharacter.BPC_InventoryComponent` (`self.As CH Survival Character`))))
  (bind _asbp_weapon_base (cast `/Game/Somewhere/Objects/Items/Weapons/BP_WeaponBase` (`/Game/Somewhere/Core/Player/Inventory/BPC_InventoryComponent.Current Holdable` (`/Game/Somewhere/Core/Player/CH_SurvivalCharacter.BPC_InventoryComponent` (`self.As CH Survival Character`)))))
  (set `local.Weapon Base` _asbp_weapon_base)
  (set `local.L Requied Ammo` (- (`/Game/Somewhere/Core/Holdable/BP_Gun.AmmoMagazinSize` (`local.Weapon Base`)) (`.CustomInteger` (break `InventoryItem` (`/Game/Somewhere/Core/Holdable/BP_Holdable.Inventory Item` (`local.Weapon Base`))))))
  (bind _output_get (set `local.L Cached Indexes` (`ItemContainer.FindAllCellsWithItem` _main_container (`local.Ammo ID`))))
  (for _array_element _output_get
    (bind _output_get_2 (set `local.L Modified Requied Ammo` (- (`local.L Requied Ammo`) (`local.L Reloaded Amount`))))
    (if (> _output_get_2 0)
      (bind (_id _amount) (break `InventoryItem` (`ItemContainer.GetCell` _main_container _array_element)))
      (if (> _amount _l_modified_requied_ammo)
        (bind _output_get_3 (set `local.L Actual Reloaded Amount` _l_modified_requied_ammo))
        (`ItemContainer.RemoveItemAmountFromCell` _main_container _array_element _output_get_3)
        (set `local.L Reloaded Amount` (+ _l_modified_requied_ammo (`local.L Reloaded Amount`)))
        (else
          (bind _output_get_4 (set `local.L Actual Reloaded Amount` _amount))
          (`ItemContainer.RemoveItemAmountFromCell` _main_container _array_element _output_get_4)
          (set `local.L Reloaded Amount` (+ (`local.L Reloaded Amount`) (`local.L Actual Reloaded Amount`)))))
      (else
        (break))))
  (if (> (`local.L Reloaded Amount`) 0)
    (return true (- (`/Game/Somewhere/Core/Holdable/BP_Gun.AmmoMagazinSize` (`local.Weapon Base`)) (- (`local.L Requied Ammo`) (`local.L Reloaded Amount`))))
    (else
      (return false 0))))