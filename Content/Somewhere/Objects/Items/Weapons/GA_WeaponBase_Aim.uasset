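; Gameplay ability for aiming a weapon on the survival character.
; On activation it shortens and tightens the camera boom and enables the CM_Aim camera modifier, adding it if missing.
; It ends on the Aim.InputCompleted gameplay event, restoring the boom and disabling the stored modifier.
; An ApplyDamage function does a forward sphere trace dealing point damage once per actor, but nothing here calls it.
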(event `self.K2_ActivateAbility`
  (bind _returnvalue (`GameplayStatics.GetPlayerCameraManager` 0))
  (bind _cameraboom (`/Game/Somewhere/Core/Player/CH_SurvivalCharacter.CameraBoom` (`self.As CH Survival Character`)))
  (`|ExecutionSequence`
    (:`then_0`
      ;[0 0 0] Рефы
      (bind _ascharacter (cast `Character` (`self.GetAvatarActorFromActorInfo`)))
      (bind _output_get (set `self.Character` _ascharacter))
      (bind _asplayer_controller (cast `PlayerController` (`Pawn.GetController` _output_get)))
      (set `self.Player Controller` _asplayer_controller)
      (bind _asch_survival_character (cast `/Game/Somewhere/Core/Player/CH_SurvivalCharacter` (`self.Character`)))
      (set `self.As CH Survival Character` _asch_survival_character))
    (:`then_1`
      ;[0 0 0] Смещение камеры
      (set `SpringArmComponent.CameraRotationLagSpeed` 40.0 _cameraboom)
      (set `SpringArmComponent.CameraLagSpeed` 30.0 _cameraboom)
      (set `SpringArmComponent.TargetArmLength` 80.0 _cameraboom)
      (bind _returnvalue_2 (`PlayerCameraManager.FindCameraModifierByClass` _returnvalue "/Game/Somewhere/Core/Camera/CM_Aim.CM_Aim_C"))
      (`/Engine/EditorBlueprintResources/StandardMacros.IsValid` _returnvalue_2
        (:`Is Valid`
          (`CameraModifier.EnableModifier` _returnvalue_2))
        (:`Is Not Valid`
          (bind _returnvalue_3 (`PlayerCameraManager.AddNewCameraModifier` _returnvalue "/Game/Somewhere/Core/Camera/CM_Aim.CM_Aim_C"))
          (bind _output_get_2 (set `self.Camera Mod` _returnvalue_3))
          (`CameraModifier.EnableModifier` _output_get_2))))
    (:`then_3`
      (`AbilityTask_WaitGameplayEvent.WaitGameplayEvent` (struct :`TagName` "GameplayAbility.Weapon.Aim.InputCompleted") null
        (:`EventReceived`
          (`self.K2_EndAbility`))))))

(event `self.K2_OnEndAbility`
  (params (bWasCancelled :type Boolean))
  (bind _camera_mod (`self.Camera Mod`))
  (bind _cameraboom (`/Game/Somewhere/Core/Player/CH_SurvivalCharacter.CameraBoom` (`self.As CH Survival Character`)))
  (set `SpringArmComponent.CameraRotationLagSpeed` 20.0 _cameraboom)
  (set `SpringArmComponent.CameraLagSpeed` 10.0 _cameraboom)
  (set `SpringArmComponent.TargetArmLength` 230.0 _cameraboom)
  (`/Engine/EditorBlueprintResources/StandardMacros.IsValid` _camera_mod
    (:`Is Valid`
      (`CameraModifier.DisableModifier` _camera_mod false))))

(fn `Apply Damage`
  (locals (`L Damaged Actors` :type "Array of Actor Object Reference") (`L Hit Actor` :type "Actor Object Reference"))
  (bind _character (`self.Character`))
  (bind _returnvalue (+ (`Actor.K2_GetActorLocation` _character) (* (`Actor.GetActorForwardVector` _character) 90.0)))
  ;[0 0 0] Сфера дамага спереди
  (bind (_outhits _returnvalue_2) (`KismetSystemLibrary.SphereTraceMulti` _returnvalue _returnvalue 90.0 "TraceTypeQuery1" false (`|MakeArray` (`self.Character`) :!type "Actor Object Reference") "None" true (struct :`R` 1.0 :`A` 1.0) (struct :`G` 1.0 :`A` 1.0) 1.0))
  (if _returnvalue_2
    (for _array_element _outhits
      (set `local.L Hit Actor` (`.HitActor` (`GameplayStatics.BreakHitResult` _array_element)))
      ;[0 0 0] Дамажим всех, но только по одному разу
      (if (not (`KismetArrayLibrary.Array_Contains` (`local.L Damaged Actors`) (`local.L Hit Actor`)))
        (`KismetArrayLibrary.Array_AddUnique` (`local.L Damaged Actors`) (`local.L Hit Actor`))
        (`GameplayStatics.ApplyPointDamage` (`local.L Hit Actor`) 20.0 (`KismetMathLibrary.Normal` (- (`Actor.K2_GetActorLocation` (`local.L Hit Actor`)) (`Actor.K2_GetActorLocation` (`self.Character`)))) (`GameplayStatics.MakeHitResult` false) (`self.Player Controller`) (`self.Character`) "/Game/Somewhere/Core/DamageTypes/DT_Bullet.DT_Bullet_C")))))