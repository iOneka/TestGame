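; Gameplay ability for the semi-automatic pistol's Hold action; this graph holds its damage step.
; ApplyDamage runs a zero-length multi sphere trace on the Visibility channel just in front of the character, ignoring the character itself.
; Each unique hit actor takes fixed bullet-type point damage once, directed away from the character, so the pistol hits a close-range area rather than along a bullet line.
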(fn `Apply Damage`
  (locals (`L Damaged Actors` :type "Array of Actor Object Reference") (`L Hit Actor` :type "Actor Object Reference"))
  (bind _character (`self.Character`))
  (bind _returnvalue (+ (`Actor.K2_GetActorLocation` _character) (* (`Actor.GetActorForwardVector` _character) 90.0)))
  ;[0 0 0] Сфера дамага спереди
  (bind (_outhits _returnvalue_2) (`KismetSystemLibrary.SphereTraceMulti` _returnvalue _returnvalue 90.0 "TraceTypeQuery1" false (`|MakeArray` (`self.Character`) :!type "Actor Object Reference") "None" true (struct :`R` 1.0 :`A` 1.0) (struct :`G` 1.0 :`A` 1.0) 1.0))
  (if _returnvalue_2
    (for _array_element _outhits
      (set `local.L Hit Actor` (`.HitActor` (`GameplayStatics.BreakHitResult` _array_element)))
      ;[0 0 0] Дамажим всех, но только по одному разу
      (if (not (`KismetArrayLibrary.Array_Contains` (`local.L Damaged Actors`) (`local.L Hit Actor`)))
        (`KismetArrayLibrary.Array_AddUnique` (`local.L Damaged Actors`) (`local.L Hit Actor`))
        (`GameplayStatics.ApplyPointDamage` (`local.L Hit Actor`) 20.0 (`KismetMathLibrary.Normal` (- (`Actor.K2_GetActorLocation` (`local.L Hit Actor`)) (`Actor.K2_GetActorLocation` (`self.Character`)))) (`GameplayStatics.MakeHitResult` false) (`self.Player Controller`) (`self.Character`) "/Game/Somewhere/Core/DamageTypes/DT_Bullet.DT_Bullet_C")))))