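; Base equipped gun item that attaches to the character's hand and takes its ammo count from the inventory cell.
; The server grants fire, aim, reload and hold GAS abilities, which Enhanced Input triggers with ammo checks and cooldown gates.
; Gameplay messages update ammo and crosshair UI.
; On local standalone/client Tick, camera-then-muzzle traces offset the crosshair and set an obstacle tag when the muzzle's aim angle is too wide.
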(event `EnhancedInput|/Game/Somewhere/Core/Input/Actions/Gun/IA_Gun_Fire`
  (params (ActionValue :type Boolean) (ElapsedSeconds :type "Float (double-precision)") (TriggeredSeconds :type "Float (double-precision)") (InputAction :type "InputAction Object Reference" :default "/Game/Somewhere/Core/Input/Actions/Gun/IA_Gun_Fire.IA_Gun_Fire"))
  (:`Triggered`
    (`self.Gun Fire Triggered`))
  (:`Started`
    (`self.Gun Fire Started`)))

(event `Gun Fire Triggered`
  (if (> (`.CustomInteger` (break `InventoryItem` (`self.Inventory Item`))) 0)
    (if (not (`/Game/Somewhere/Core/Player/CH_SurvivalCharacter.Is Jumping` (`self.Owner as Survival Character`)))
      (`/Engine/EditorBlueprintResources/StandardMacros.DoOnce` false :!label _label
        (:`Completed`
          (`|ExecutionSequence`
            (:`then_0`
              (bind _returnvalue (`AbilitySystemComponent.TryActivateAbility` (`AbilitySystemBlueprintLibrary.GetAbilitySystemComponent` (`self.Owner as Character`)) (`self.Fire Ability`) true))
              (if _returnvalue
                (`SkeletalMeshComponent.PlayAnimation` (`self.SkeletalMesh`) (`self.Weapon Fire Anim`) false)
                (set `self.Is Not First Fire` true)
                (`self.SERVER ChangeIsFirstFire` true)
                (`KismetSystemLibrary.RetriggerableDelay` 0.7)
                (`self.SERVER ChangeIsFirstFire` false)
                (set `self.Is Not First Fire` false)))
            (:`then_1`
              (`GameplayMessageSubsystem.K2_BroadcastMessage` (subsystem `GameplayMessageSubsystem`) (struct :`TagName` "GameplayMessage.UpdateAmmo") (make `/Game/Somewhere/UIv2/Widgets/Gameplay/HUD/Weapon/S_AmmoUpdate` (`.CustomInteger` (break `InventoryItem` (`self.Inventory Item`))) (`self.AmmoMagazinSize`)))
              (`KismetSystemLibrary.Delay` (`self.FireDelay Duration`))
              (goto _label :!via `Reset`))))))))

(event `Gun Fire Started`
  (if (not (> (`.CustomInteger` (break `InventoryItem` (`self.Inventory Item`))) 0))
    (`GameplayMessageSubsystem.K2_BroadcastMessage` (subsystem `GameplayMessageSubsystem`) (struct :`TagName` "GameplayMessage.NotEnoughAmmo") (make `EmptyPayload`))
    (`GameplayStatics.PlaySoundAtLocation` (`self.EmptyMagSound`) (`SceneComponent.K2_GetComponentLocation` (`self.SkeletalMesh`)) (struct) 1.0 1.0 0.0 null null null null)))

(event `self.ReceiveBeginPlay`
  (bind (_returnvalue_x _returnvalue_y) (`KismetMathLibrary.BreakVector2D` (`WidgetLayoutLibrary.GetViewportSize`)))
  (bind _returnvalue (subsystem `GameplayMessageSubsystem`))
  (bind (_inventory_item_id _inventory_item_amount _inventory_item_cell _inventory_item_custominteger) (break `InventoryItem` (`self.Inventory Item`)))
  (bind _offset_location (`KismetMathLibrary.BreakTransform` (`self.Offset`)))
  (bind (_offset_location_2 _offset_rotation) (`KismetMathLibrary.BreakTransform` (`self.Offset`)))
  (`parent.ReceiveBeginPlay`)
  ;[0 0 0] взлом жопы
  (`|ExecutionSequence`
    (:`then_0`
      (`|ExecutionSequence`
        (:`then_0`
          ;[0 0 0] Крепим к руке
          (`self.K2_AttachToComponent` (`Character.Mesh` (`self.Owner as Character`)) (`self.Socket Name`) "SnapToTarget" "SnapToTarget" "SnapToTarget")
          ;[0 0 0] Точное положение
          (`SceneComponent.K2_AddRelativeLocation` (`self.Item Mesh`) _offset_location false false)
          (`SceneComponent.K2_AddRelativeRotation` (`self.Item Mesh`) _offset_rotation false false)
          (set `self.Skeletal Mesh` (`self.SkeletalMesh`))
          ;[0 0 0] Берем данные из инвенторя
          (set `self.Inventory Item` (`ItemContainer.GetCell` (`/Game/Somewhere/Core/Player/Inventory/BPC_InventoryComponent.Main Container` (`/Game/Somewhere/Core/Player/CH_SurvivalCharacter.BPC_InventoryComponent` (`self.Owner as Survival Character`))) (`self.Cell Item`)))
          (set `self.Mobile?` (`SomewhereStatics.IsMobilePlatform`))
          ;[0 0 0] Анимация взятия
          (bind _equip_animation (`self.Equip Animation`)
            (:`then`
              (`|PlayMontage` (`Character.Mesh` (`self.Owner as Character`)) _equip_animation))
            (:`else`)))))
    (:`then_1`
      (`/Engine/EditorBlueprintResources/ActorMacros.Switch Has Authority`
        (:`Authority`
          (`|ExecutionSequence`
            (:`then_0`
              (bind _returnvalue_2 (`AbilitySystemComponent.K2_GiveAbility` (`AbilitySystemBlueprintLibrary.GetAbilitySystemComponent` (`self.Owner as Character`)) (`self.Fire Ability Class`) 0 -1))
              (set `self.Fire Ability` _returnvalue_2)
              (bind _returnvalue_3 (`AbilitySystemComponent.K2_GiveAbility` (`AbilitySystemBlueprintLibrary.GetAbilitySystemComponent` (`self.Owner as Character`)) (`self.Aim Ability Class`) 0 -1))
              (set `self.Aim Ability` _returnvalue_3)
              (bind _returnvalue_4 (`AbilitySystemComponent.K2_GiveAbility` (`AbilitySystemBlueprintLibrary.GetAbilitySystemComponent` (`self.Owner as Character`)) (`self.Reload Ability Class`) 0 -1))
              (set `self.Reload Ability` _returnvalue_4)
              (bind _returnvalue_5 (`AbilitySystemComponent.K2_GiveAbility` (`AbilitySystemBlueprintLibrary.GetAbilitySystemComponent` (`self.Owner as Character`)) (`self.Hold Ability Class`) 0 -1))
              (bind _output_get (set `self.Hold Ability` _returnvalue_5))
              (`AbilitySystemComponent.TryActivateAbility` (`AbilitySystemBlueprintLibrary.GetAbilitySystemComponent` (`self.Owner as Character`)) _output_get true))))))
    (:`then_2`
      (if (`Pawn.IsLocallyControlled` (`self.Owner as Character`))
        (`|ExecutionSequence`
          (:`then_0`
            ;[0 0 0] Слушаем действия внематочно и сосредодрочено
            (`EnhancedInputSubsystemInterface.AddMappingContext` (pcsubsystem `EnhancedInputLocalPlayerSubsystem` (`GameplayStatics.GetPlayerController` 0)) "/Game/Somewhere/Core/Input/Actions/Gun/IMC_Gun.IMC_Gun" 1 (struct))
            (`self.EnableInput` (`GameplayStatics.GetPlayerController` 0))
            (`GameplayMessageSubsystem.K2_BroadcastMessage` _returnvalue (struct :`TagName` "GameplayMessage.UpdateAmmo") (make `/Game/Somewhere/UIv2/Widgets/Gameplay/HUD/Weapon/S_AmmoUpdate` _inventory_item_custominteger (`self.AmmoMagazinSize`)))
            (`GameplayMessageSubsystem.K2_BroadcastMessage` _returnvalue (struct :`TagName` "GameplayMessage.VisibilityWidgetAmmo") (make `/Game/Somewhere/UIv2/Widgets/Gameplay/HUD/Weapon/S_AmmoVisibility` true))
            ;[0 0 0] For crosshire, half screen
            (set `self.HalfScreenSizeX` (/ _returnvalue_x 2.0))
            (set `self.HalfScreenSizeY` (/ _returnvalue_y 2.0))
            (set `self.ArrayTagObstacle` (`|MakeArray` (struct :`TagName` "GameplayAbility.Weapon.Fire.Obstacle") :!type "GameplayTag Structure"))))))))

(event `EnhancedInput|/Game/Somewhere/Core/Input/Actions/Gun/IA_Gun_Aim`
  (params (ActionValue :type Boolean) (ElapsedSeconds :type "Float (double-precision)") (TriggeredSeconds :type "Float (double-precision)") (InputAction :type "InputAction Object Reference" :default "/Game/Somewhere/Core/Input/Actions/Gun/IA_Gun_Aim.IA_Gun_Aim"))
  (:`Started`
    (`/Engine/EditorBlueprintResources/StandardMacros.FlipFlop`
      (:`A`
        (`AbilitySystemComponent.TryActivateAbility` (`AbilitySystemBlueprintLibrary.GetAbilitySystemComponent` (`self.Owner as Character`)) (`self.Aim Ability`) true))
      (:`B`
        (`AbilitySystemBlueprintLibrary.SendGameplayEventToActor` (`self.Owner as Character`) (struct :`TagName` "GameplayAbility.Weapon.Aim.InputCompleted"))))))

(event `EnhancedInput|/Game/Somewhere/Core/Input/Actions/Gun/IA_Gun_Reload`
  (params (ActionValue :type Boolean) (ElapsedSeconds :type "Float (double-precision)") (TriggeredSeconds :type "Float (double-precision)") (InputAction :type "InputAction Object Reference" :default "/Game/Somewhere/Core/Input/Actions/Gun/IA_Gun_Reload.IA_Gun_Reload"))
  (:`Triggered`
    (if (!= (`.CustomInteger` (break `InventoryItem` (`self.Inventory Item`))) (`self.AmmoMagazinSize`))
      (if (`.ReturnValue` (`ItemContainer.FindAllCellsWithItem` (`/Game/Somewhere/Core/Player/Inventory/BPC_InventoryComponent.Main Container` (`/Game/Somewhere/Core/Player/CH_SurvivalCharacter.BPC_InventoryComponent` (`self.Owner as Survival Character`))) (`self.AmmunitionID`)))
        (`/Engine/EditorBlueprintResources/StandardMacros.DoOnce` false :!label _label_2
          (:`Completed`
            (`|ExecutionSequence`
              (:`then_0`
                (`AbilitySystemComponent.TryActivateAbility` (`AbilitySystemBlueprintLibrary.GetAbilitySystemComponent` (`self.Owner as Character`)) (`self.Reload Ability`) true)
                (`SkeletalMeshComponent.PlayAnimation` (`self.SkeletalMesh`) (`self.Weapon Reload Anim`) false))
              (:`then_1`
                (`KismetSystemLibrary.Delay` (`self.Reload Duration`))
                (`KismetSystemLibrary.Delay` 0.2)
                (`GameplayMessageSubsystem.K2_BroadcastMessage` (subsystem `GameplayMessageSubsystem`) (struct :`TagName` "GameplayMessage.UpdateAmmo") (make `/Game/Somewhere/UIv2/Widgets/Gameplay/HUD/Weapon/S_AmmoUpdate` (`.CustomInteger` (break `InventoryItem` (`self.Inventory Item`))) (`self.AmmoMagazinSize`)))
                (goto _label_2 :!via `Reset`)))))))))

(event `self.ReceiveEndPlay`
  (params (EndPlayReason :type "EEndPlayReason Enum" :default "Destroyed"))
  (bind _returnvalue (subsystem `GameplayMessageSubsystem`))
  ;[0 0 0] взлом жопы
  (`|ExecutionSequence`
    (:`then_0`
      (`|ExecutionSequence`))
    (:`then_1`
      (`/Engine/EditorBlueprintResources/ActorMacros.Switch Has Authority`
        (:`Authority`
          (`|ExecutionSequence`
            (:`then_0`
              ;[0 0 0] ты больше не армянин
              (`AbilitySystemComponent.ClearAbility` (`AbilitySystemBlueprintLibrary.GetAbilitySystemComponent` (`self.Owner as Character`)) (`self.Fire Ability`))
              (`AbilitySystemComponent.ClearAbility` (`AbilitySystemBlueprintLibrary.GetAbilitySystemComponent` (`self.Owner as Character`)) (`self.Aim Ability`))
              (`AbilitySystemComponent.ClearAbility` (`AbilitySystemBlueprintLibrary.GetAbilitySystemComponent` (`self.Owner as Character`)) (`self.Reload Ability`))
              (`AbilitySystemComponent.ClearAbility` (`AbilitySystemBlueprintLibrary.GetAbilitySystemComponent` (`self.Owner as Character`)) (`self.Reload Ability`))
              (`AbilitySystemComponent.ClearAbility` (`AbilitySystemBlueprintLibrary.GetAbilitySystemComponent` (`self.Owner as Character`)) (`self.Hold Ability`)))))))
    (:`then_2`
      (if (`Pawn.IsLocallyControlled` (`self.Owner as Character`))
        (`|ExecutionSequence`
          (:`then_0`
            (`GameplayMessageSubsystem.K2_BroadcastMessage` (subsystem `GameplayMessageSubsystem`) (struct :`TagName` "GameplayMessage.VisibilityWidgetAmmo") (make `/Game/Somewhere/UIv2/Widgets/Gameplay/HUD/Weapon/S_AmmoVisibility` false))
            ;[0 0 0] не Слушаем действия внематочно и сосредодрочено
            (`EnhancedInputSubsystemInterface.RemoveMappingContext` (pcsubsystem `EnhancedInputLocalPlayerSubsystem` (`GameplayStatics.GetPlayerController` 0)) "/Game/Somewhere/Core/Input/Actions/Gun/IMC_Gun.IMC_Gun" (struct))
            (`self.DisableInput` (`GameplayStatics.GetPlayerController` 0))
            (`AbilitySystemBlueprintLibrary.RemoveLooseGameplayTags` (`self.Owner as Survival Character`) (make `GameplayTagContainer` (`self.ArrayTagObstacle`)))
            (`GameplayMessageSubsystem.K2_BroadcastMessage` _returnvalue (struct :`TagName` "GameplayMessage.CrosshireObstacle") (make `/Game/Somewhere/Objects/Items/Weapons/S_CrosshireObstacle` false))
            (`GameplayMessageSubsystem.K2_BroadcastMessage` _returnvalue (struct :`TagName` "GameplayMessage.CrosshireChange") (make `/Game/Somewhere/Objects/Items/Weapons/S_ChangeCrosshire` 0.0))))))))

(event `self.ReceiveTick`
  (params (DeltaSeconds :type "Float (single-precision)"))
  (bind _returnvalue (subsystem `GameplayMessageSubsystem`))
  (bind _arraytagobstacle (`self.ArrayTagObstacle`))
  (bind (_out_hit_bblockinghit _out_hit_binitialoverlap _out_hit_time _out_hit_distance _out_hit_location) (`GameplayStatics.BreakHitResult` (`self.Out Hit`)))
  (bind _owner_as_survival_character (`self.Owner as Survival Character`))
  (bind _returnvalue_2 (`SceneComponent.K2_GetComponentLocation` (`self.Trigger`)))
  (bind _screenposition (`GameplayStatics.ProjectWorldToScreen` (`self.Owner As Player Controller`) _out_hit_location))
  (bind (_location _rotation) (`Controller.GetPlayerViewPoint` (`GameplayStatics.GetPlayerController` 0)))
  (bind _returnvalue_3 (`SceneComponent.K2_GetComponentLocation` (`self.Trigger`)))
  (bind _returnvalue_4 (`Pawn.GetController` (cast `Character` (`self.GetOwner`) :!pure true)))
  (bind _returnvalue_5 (+ _location (* (`KismetMathLibrary.Conv_RotatorToVector` _rotation) (`self.Distance`))))
  (`/Game/Somewhere/Core/Libraries/BML_BP_Somewhere.Switch Has Authority 2`
    (:`Standalone`
      _)
    (:`Client`
      _))
  (`/Engine/EditorBlueprintResources/StandardMacros.IsValid` _returnvalue_4
    (:`Is Valid`
      (if (and (`KismetSystemLibrary.IsValid` _returnvalue_4) (`Controller.IsLocalPlayerController` _returnvalue_4))
        ;[0 0 0] LineTrace до прицела
        (bind (_outhit _returnvalue_6) (`KismetSystemLibrary.LineTraceSingle` _location _returnvalue_5 "TraceTypeQuery1" false (`|MakeArray` (`self.Owner as Character`) :!type "Actor Object Reference") "None" true (struct :`G` 1.0 :`B` 0.962814 :`A` 1.0) (struct :`R` 0.985269 :`G` 0.988951 :`B` 1.0 :`A` 1.0) 10.0))
        (if _returnvalue_6
          ;[0 0 0] Выстрел в объект
          (bind (_outhit_2 _returnvalue_7) (`KismetSystemLibrary.LineTraceSingle` _returnvalue_3 (+ (* (`KismetMathLibrary.GetForwardVector` (`KismetMathLibrary.FindLookAtRotation` _returnvalue_3 (`.ImpactPoint` (`GameplayStatics.BreakHitResult` _outhit)))) (`self.Distance`)) _returnvalue_3) "TraceTypeQuery1" false (`|MakeArray` (`self.Owner as Character`) :!type "Actor Object Reference") "None" true (struct :`R` 1.0 :`B` 0.730776 :`A` 1.0)))
          (bind _output_get (set `self.Out Hit` _outhit_2))
          (set `self.OutHitBool` _returnvalue_7)
          (bind (_returnvalue_roll _returnvalue_pitch _returnvalue_yaw) (`KismetMathLibrary.BreakRotator` (`KismetMathLibrary.FindRelativeLookAtRotation` (`SceneComponent.K2_GetComponentToWorld` (`self.Trigger`)) (`KismetMathLibrary.SelectVector` (`.ImpactPoint` (`GameplayStatics.BreakHitResult` _output_get)) (`.TraceEnd` (`GameplayStatics.BreakHitResult` _output_get)) (!= (`.ImpactPoint` (`GameplayStatics.BreakHitResult` _output_get)) (0.0 0.0 0.0))))))
          (if (and (< (`KismetMathLibrary.Abs` _returnvalue_yaw) 30.0) (< (`KismetMathLibrary.Abs` _returnvalue_pitch) 30.0))
            (`AbilitySystemBlueprintLibrary.RemoveLooseGameplayTags` _owner_as_survival_character (make `GameplayTagContainer` _arraytagobstacle) :!label _label_3)
            (`GameplayMessageSubsystem.K2_BroadcastMessage` _returnvalue (struct :`TagName` "GameplayMessage.CrosshireObstacle") (make `/Game/Somewhere/Objects/Items/Weapons/S_CrosshireObstacle` false))
            ;[0 0 0] CrosshireChanges
            (if (`self.OutHitBool`)
              (if (< _out_hit_distance 1500.0)
                (`GameplayMessageSubsystem.K2_BroadcastMessage` (subsystem `GameplayMessageSubsystem`) (struct :`TagName` "GameplayMessage.CrosshireChange") (make `/Game/Somewhere/Objects/Items/Weapons/S_ChangeCrosshire` (- (`KismetMathLibrary.BreakVector2D` _screenposition) (`self.HalfScreenSizeX`)) (- (`.Y` (`KismetMathLibrary.BreakVector2D` _screenposition)) (`self.HalfScreenSizeY`))))
                (else
                  (`GameplayMessageSubsystem.K2_BroadcastMessage` (subsystem `GameplayMessageSubsystem`) (struct :`TagName` "GameplayMessage.CrosshireChange") (make `/Game/Somewhere/Objects/Items/Weapons/S_ChangeCrosshire` 0.0) :!label _label_4)))
              (else
                (goto _label_4)))
            (else
              (if (not (> (`AbilitySystemComponent.GetGameplayTagCount` (`SomewhereCharacter.AbilitySystemComponent` (`self.Owner as Survival Character`)) (struct :`TagName` "GameplayAbility.Weapon.Fire.Obstacle")) 0)) :!label _label_5
                (`AbilitySystemBlueprintLibrary.AddLooseGameplayTags` _owner_as_survival_character (make `GameplayTagContainer` _arraytagobstacle))
                (`GameplayMessageSubsystem.K2_BroadcastMessage` _returnvalue (struct :`TagName` "GameplayMessage.CrosshireObstacle") (make `/Game/Somewhere/Objects/Items/Weapons/S_CrosshireObstacle` true)))))
          (else
            ;[0 0 0] Выстрел в воздух
            (bind (_outhit_3 _returnvalue_8) (`KismetSystemLibrary.LineTraceSingle` _returnvalue_2 (+ (* (`KismetMathLibrary.GetForwardVector` (`KismetMathLibrary.FindLookAtRotation` _returnvalue_2 _returnvalue_5)) (`self.Distance`)) _returnvalue_2) "TraceTypeQuery1" false (`|MakeArray` (`self.Owner as Character`) :!type "Actor Object Reference") "None" true (struct :`R` 0.358979 :`G` 1.0 :`A` 1.0) (struct :`R` 0.99765 :`G` 1.0 :`A` 1.0)))
            (bind _output_get_2 (set `self.Out Hit` _outhit_3))
            (set `self.OutHitBool` _returnvalue_8)
            (bind (_returnvalue_roll_2 _returnvalue_pitch_2 _returnvalue_yaw_2) (`KismetMathLibrary.BreakRotator` (`KismetMathLibrary.FindRelativeLookAtRotation` (`SceneComponent.K2_GetComponentToWorld` (`self.Trigger`)) (`KismetMathLibrary.SelectVector` (`.ImpactPoint` (`GameplayStatics.BreakHitResult` _output_get_2)) (`.TraceEnd` (`GameplayStatics.BreakHitResult` _output_get_2)) (!= (`.ImpactPoint` (`GameplayStatics.BreakHitResult` _output_get_2)) (0.0 0.0 0.0))))))
            (if (and (< (`KismetMathLibrary.Abs` _returnvalue_pitch_2) 30.0) (< (`KismetMathLibrary.Abs` _returnvalue_yaw_2) 30.0))
              (goto _label_3)
              (else
                (goto _label_5)))))))))

(fn `OnRep_CurrentAmmo`)

(fn `UserConstructionScript`
  (`parent.UserConstructionScript`))