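; Gameplay ability for the machete's melee swing.
; On activation it plays a random montage from a moving or standing pair chosen by character speed, using PlayMontage when locally controlled and PlayMontageAndWait otherwise.
; Each swing starts a client camera shake, then after a short delay calls ApplyDamage.
; ApplyDamage sphere-traces in front of the character and deals melee point damage once per hit actor.
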(event `self.K2_ActivateAbility`
  (`|ExecutionSequence`
    (:`then_0`
      ;[0 0 0] Рефы
      (bind _ascharacter (cast `Character` (`self.GetAvatarActorFromActorInfo`)))
      (bind _output_get (set `self.Character` _ascharacter))
      (bind _asch_survival_character (cast `/Game/Somewhere/Core/Player/CH_SurvivalCharacter` _output_get))
      (set `self.As CH Survival Character` _asch_survival_character)
      (bind _asplayer_controller (cast `PlayerController` (`Pawn.GetController` _output_get)))
      (set `self.Player Controller` _asplayer_controller))
    (:`then_1`
      (set `self.Sweep Animation` (select `bool` (`KismetMathLibrary.RandomBool`) :`false` "/Game/Somewhere/Core/Player/Animations/NewAnimationsMixamo/Armyanin/AM_Sword_Hit_1.AM_Sword_Hit_1" :`true` "/Game/Somewhere/Core/Player/Animations/NewAnimationsMixamo/Armyanin/AM_Sword_Hit_2.AM_Sword_Hit_2" :!type "AnimMontage Object Reference"))
      ;[0 0 0] Анимация
      (set `self.Sweep Animation Velocity` (select `bool` (`KismetMathLibrary.RandomBool`) :`false` "/Game/Somewhere/Core/Player/Animations/NewAnimationsMixamo/Armyanin/AM_Sword_Hit_3.AM_Sword_Hit_3" :`true` "/Game/Somewhere/Core/Player/Animations/NewAnimationsMixamo/Armyanin/AM_Sword_Hit_4.AM_Sword_Hit_4" :!type "AnimMontage Object Reference"))
      (if (> (`/Game/Somewhere/Core/Player/CH_SurvivalCharacter.Speed` (`self.As CH Survival Character`)) 0.0)
        (`self.IsLocallyControlled`
          (:`True`
            (`|PlayMontage` (`Character.Mesh` (`self.Character`)) (`self.Sweep Animation Velocity`) 1.5
              (:`then`
                _)))
          (:`False`
            (`AbilityTask_PlayMontageAndWait.CreatePlayMontageAndWaitProxy` "None" (`self.Sweep Animation Velocity`) 1.5
              (:`then`
                _))))
        (else
          (`self.IsLocallyControlled`
            (:`True`
              (`|PlayMontage` (`Character.Mesh` (`self.Character`)) (`self.Sweep Animation`) 1.5
                (:`then`
                  _)))
            (:`False`
              (`AbilityTask_PlayMontageAndWait.CreatePlayMontageAndWaitProxy` "None" (`self.Sweep Animation`) 1.5
                (:`then`
                  _))))))
      (`PlayerController.ClientStartCameraShake` :`self` (`self.Player Controller`) :`Shake` "/Game/Somewhere/Core/Camera/Attack_CameraShake.Attack_CameraShake_C" :`Scale` 0.5)
      (`KismetSystemLibrary.Delay` 0.3)
      (`self.Apply Damage`))))

(fn `Apply Damage`
  (locals (`L Damaged Actors` :type "Array of Actor Object Reference") (`L Hit Actor` :type "Actor Object Reference") (NewLocalVar :type "HitResult Structure"))
  (bind (_newlocalvar_bblockinghit _newlocalvar_binitialoverlap _newlocalvar_time _newlocalvar_distance _newlocalvar_location _newlocalvar_impactpoint _newlocalvar_normal _newlocalvar_impactnormal _newlocalvar_physmat _newlocalvar_hitactor _newlocalvar_hitcomponent _newlocalvar_hitbonename _newlocalvar_bonename _newlocalvar_hititem _newlocalvar_elementindex _newlocalvar_faceindex _newlocalvar_tracestart _newlocalvar_traceend) (`GameplayStatics.BreakHitResult` (`local.NewLocalVar`)))
  (bind _character (`self.Character`))
  (bind _returnvalue (+ (`Actor.K2_GetActorLocation` _character) (* (`Actor.GetActorForwardVector` _character) 90.0)))
  ;[0 0 0] Сфера дамага спереди
  (bind (_outhits _returnvalue_2) (`KismetSystemLibrary.SphereTraceMulti` _returnvalue _returnvalue 90.0 "TraceTypeQuery1" false (`|MakeArray` (`self.Character`) :!type "Actor Object Reference") "None" true (struct :`R` 1.0 :`A` 1.0) (struct :`G` 1.0 :`A` 1.0) 1.0))
  (if _returnvalue_2
    (for _array_element _outhits
      (set `local.NewLocalVar` _array_element)
      (set `local.L Hit Actor` (`.HitActor` (`GameplayStatics.BreakHitResult` _array_element)))
      ;[0 0 0] Дамажим всех, но только по одному разу
      (if (not (`KismetArrayLibrary.Array_Contains` (`local.L Damaged Actors`) (`local.L Hit Actor`)))
        (`KismetArrayLibrary.Array_AddUnique` (`local.L Damaged Actors`) (`local.L Hit Actor`))
        (`/Engine/EditorBlueprintResources/StandardMacros.IsValid` (`local.L Hit Actor`)
          (:`Is Valid`
            (`GameplayStatics.ApplyPointDamage` (`local.L Hit Actor`) 20.0 (`KismetMathLibrary.Normal` (- (`Actor.K2_GetActorLocation` (`local.L Hit Actor`)) (`Actor.K2_GetActorLocation` (`self.Character`)))) (`GameplayStatics.MakeHitResult` _newlocalvar_bblockinghit _newlocalvar_binitialoverlap _newlocalvar_time _newlocalvar_distance _newlocalvar_location _newlocalvar_location _newlocalvar_normal _newlocalvar_impactnormal _newlocalvar_physmat _newlocalvar_hitactor _newlocalvar_hitcomponent _newlocalvar_hitbonename _newlocalvar_bonename _newlocalvar_hititem _newlocalvar_elementindex _newlocalvar_faceindex _newlocalvar_tracestart _newlocalvar_traceend) (`self.Player Controller`) (`self.Character`) "/Game/Somewhere/Core/DamageTypes/DT_Melee.DT_Melee_C")))))))