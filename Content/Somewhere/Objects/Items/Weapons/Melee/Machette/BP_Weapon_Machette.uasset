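; Machete melee weapon item that attaches to the owning character's hand socket and attacks through a Gameplay Ability.
; On BeginPlay it applies an offset, plays the equip montage, grants GA_Weapon_Machette on authority and adds the melee input mapping for the local player.
; Attack input activates the granted ability, throttled by a DoOnce and Delay cooldown.
; EndPlay clears the ability on authority and removes the local input setup.
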(event `EnhancedInput|/Game/Somewhere/Core/Input/Actions/Melee/IA_MeleeWeapon_Attack`
  (params (ActionValue :type Boolean) (ElapsedSeconds :type "Float (double-precision)") (TriggeredSeconds :type "Float (double-precision)") (InputAction :type "InputAction Object Reference" :default "/Game/Somewhere/Core/Input/Actions/Melee/IA_MeleeWeapon_Attack.IA_MeleeWeapon_Attack"))
  (:`Started`
    ;[0 0 0] Задержка между взмахами
    (`/Engine/EditorBlueprintResources/StandardMacros.DoOnce` false :!label _label
      (:`Completed`
        (`|ExecutionSequence`
          (:`then_0`
            (`AbilitySystemComponent.TryActivateAbility` (`AbilitySystemBlueprintLibrary.GetAbilitySystemComponent` (`self.Owner as Character`)) (`self.Sweep Ability`) true))
          (:`then_1`
            (`KismetSystemLibrary.Delay` 0.5)
            (goto _label :!via `Reset`)))))))

(event `EnhancedInput|/Game/Somewhere/Core/Input/Actions/Gun/IA_Gun_Aim`
  (params (ActionValue :type Boolean) (ElapsedSeconds :type "Float (double-precision)") (TriggeredSeconds :type "Float (double-precision)") (InputAction :type "InputAction Object Reference" :default "/Game/Somewhere/Core/Input/Actions/Gun/IA_Gun_Aim.IA_Gun_Aim")))

(event `self.ReceiveBeginPlay`
  (bind (_offset_location _offset_rotation) (`KismetMathLibrary.BreakTransform` (`self.Offset`)))
  (bind _offset_location_2 (`KismetMathLibrary.BreakTransform` (`self.Offset`)))
  (`parent.ReceiveBeginPlay`)
  ;[0 0 0] взлом жопы
  (`|ExecutionSequence`
    (:`then_0`
      (`|ExecutionSequence`
        (:`then_0`
          ;[0 0 0] Крепим меч к руке
          (`self.K2_AttachToComponent` (`Character.Mesh` (`self.Owner as Character`)) "Meele_socket" "SnapToTarget" "SnapToTarget" "SnapToTarget")
          ;[0 0 0] Точное положение
          (`SceneComponent.K2_AddRelativeLocation` (`self.Item Mesh`) _offset_location_2 false false)
          (`SceneComponent.K2_AddRelativeRotation` (`self.Item Mesh`) _offset_rotation false false)
          ;[0 0 0] Анимация взятия
          (bind _equip_animation (`self.Equip Animation`)
            (:`then`
              (`|PlayMontage` (`Character.Mesh` (`self.Owner as Character`)) _equip_animation))
            (:`else`)))))
    (:`then_1`
      (`/Engine/EditorBlueprintResources/ActorMacros.Switch Has Authority`
        (:`Authority`
          (`|ExecutionSequence`
            (:`then_0`
              ;[0 0 0] +100 к владению одноручками
              (bind _returnvalue (`AbilitySystemComponent.K2_GiveAbility` (`AbilitySystemBlueprintLibrary.GetAbilitySystemComponent` (`self.Owner as Character`)) "/Game/Somewhere/Objects/Items/Weapons/Melee/Machette/GA_Weapon_Machette.GA_Weapon_Machette_C" 0 -1))
              (set `self.Sweep Ability` _returnvalue))))))
    (:`then_2`
      (if (`Pawn.IsLocallyControlled` (`self.Owner as Character`))
        (`|ExecutionSequence`
          (:`then_0`
            ;[0 0 0] Слушаем действия внематочно и сосредодрочено
            (`EnhancedInputSubsystemInterface.AddMappingContext` (pcsubsystem `EnhancedInputLocalPlayerSubsystem` (`GameplayStatics.GetPlayerController` 0)) "/Game/Somewhere/Core/Input/Actions/Melee/IMC_MeleeWeapon.IMC_MeleeWeapon" 1 (struct))
            (`self.EnableInput` (`GameplayStatics.GetPlayerController` 0))))))))

(event `EnhancedInput|/Game/Somewhere/Core/Input/Actions/Gun/IA_Gun_Reload`
  (params (ActionValue :type Boolean) (ElapsedSeconds :type "Float (double-precision)") (TriggeredSeconds :type "Float (double-precision)") (InputAction :type "InputAction Object Reference" :default "/Game/Somewhere/Core/Input/Actions/Gun/IA_Gun_Reload.IA_Gun_Reload")))

(event `self.ReceiveEndPlay`
  (params (EndPlayReason :type "EEndPlayReason Enum" :default "Destroyed"))
  ;[0 0 0] взлом жопы
  (`|ExecutionSequence`
    (:`then_0`
      (`|ExecutionSequence`))
    (:`then_1`
      (`/Engine/EditorBlueprintResources/ActorMacros.Switch Has Authority`
        (:`Authority`
          (`|ExecutionSequence`
            (:`then_0`
              ;[0 0 0] ты больше не армянин
              (`AbilitySystemComponent.ClearAbility` (`AbilitySystemBlueprintLibrary.GetAbilitySystemComponent` (`self.Owner as Character`)) (`self.Sweep Ability`)))))))
    (:`then_2`
      (if (`Pawn.IsLocallyControlled` (`self.Owner as Character`))
        (`|ExecutionSequence`
          (:`then_0`
            ;[0 0 0] не Слушаем действия внематочно и сосредодрочено
            (`EnhancedInputSubsystemInterface.RemoveMappingContext` (pcsubsystem `EnhancedInputLocalPlayerSubsystem` (`GameplayStatics.GetPlayerController` 0)) "/Game/Somewhere/Core/Input/Actions/Melee/IMC_MeleeWeapon.IMC_MeleeWeapon" (struct))
            (`self.DisableInput` (`GameplayStatics.GetPlayerController` 0))))))))

(fn `UserConstructionScript`
  (`parent.UserConstructionScript`))