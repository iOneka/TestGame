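; Bizon weapon Blueprint in the Handguns folder that handles firing input, with separate paths for mobile and other platforms.
; Mobile fires on GunFireTriggered, others on GunFireStarted, both gated by ammo, jumping and a DoOnce reset after the fire delay.
; Shots activate a GAS fire ability, play the weapon animation and set a server-synced not-first-fire flag cleared by a retriggerable delay.
; Gameplay messages broadcast ammo updates and empty-magazine warnings, the latter with a sound.
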(event `self.Gun Fire Triggered`
  (if (`self.Mobile?`)
    (if (> (`.CustomInteger` (break `InventoryItem` (`self.Inventory Item`))) 0)
      (if (not (`/Game/Somewhere/Core/Player/CH_SurvivalCharacter.Is Jumping` (`self.Owner as Survival Character`)))
        (`/Engine/EditorBlueprintResources/StandardMacros.DoOnce` false :!label _label
          (:`Completed`
            (`|ExecutionSequence`
              (:`then_0`
                (bind _returnvalue (`AbilitySystemComponent.TryActivateAbility` (`AbilitySystemBlueprintLibrary.GetAbilitySystemComponent` (`self.Owner as Character`)) (`self.Fire Ability`) true))
                (if _returnvalue
                  (`SkeletalMeshComponent.PlayAnimation` (`self.SkeletalMesh`) (`self.Weapon Fire Anim`) false)
                  (set `self.Is Not First Fire` true)
                  (`self.SERVER ChangeIsFirstFire` true)
                  (`KismetSystemLibrary.RetriggerableDelay` 0.7)
                  (`self.SERVER ChangeIsFirstFire` false)
                  (set `self.Is Not First Fire` false)))
              (:`then_1`
                (`GameplayMessageSubsystem.K2_BroadcastMessage` (subsystem `GameplayMessageSubsystem`) (struct :`TagName` "GameplayMessage.UpdateAmmo") (make `/Game/Somewhere/UIv2/Widgets/Gameplay/HUD/Weapon/S_AmmoUpdate` (`.CustomInteger` (break `InventoryItem` (`self.Inventory Item`))) (`self.AmmoMagazinSize`)))
                (`KismetSystemLibrary.Delay` (`self.FireDelay Duration`))
                (goto _label :!via `Reset`)))))))))

(event `self.Gun Fire Started`
  (if (`self.Mobile?`)
    (if (not (> (`.CustomInteger` (break `InventoryItem` (`self.Inventory Item`))) 0))
      (`GameplayMessageSubsystem.K2_BroadcastMessage` (subsystem `GameplayMessageSubsystem`) (struct :`TagName` "GameplayMessage.NotEnoughAmmo") (make `EmptyPayload`))
      (`GameplayStatics.PlaySoundAtLocation` (`self.EmptyMagSound`) (`SceneComponent.K2_GetComponentLocation` (`self.SkeletalMesh`)) (struct) 1.0 1.0 0.0 null null null null))
    (elif (> (`.CustomInteger` (break `InventoryItem` (`self.Inventory Item`))) 0)
      (if (not (`/Game/Somewhere/Core/Player/CH_SurvivalCharacter.Is Jumping` (`self.Owner as Survival Character`)))
        (`/Engine/EditorBlueprintResources/StandardMacros.DoOnce` false :!label _label_2
          (:`Completed`
            (`|ExecutionSequence`
              (:`then_0`
                (bind _returnvalue (`AbilitySystemComponent.TryActivateAbility` (`AbilitySystemBlueprintLibrary.GetAbilitySystemComponent` (`self.Owner as Character`)) (`self.Fire Ability`) true))
                (if _returnvalue
                  (`SkeletalMeshComponent.PlayAnimation` (`self.SkeletalMesh`) (`self.Weapon Fire Anim`) false)
                  (set `self.Is Not First Fire` true)
                  (`self.SERVER ChangeIsFirstFire` true)
                  (`KismetSystemLibrary.RetriggerableDelay` 0.7)
                  (`self.SERVER ChangeIsFirstFire` false)
                  (set `self.Is Not First Fire` false)))
              (:`then_1`
                (`GameplayMessageSubsystem.K2_BroadcastMessage` (subsystem `GameplayMessageSubsystem`) (struct :`TagName` "GameplayMessage.UpdateAmmo") (make `/Game/Somewhere/UIv2/Widgets/Gameplay/HUD/Weapon/S_AmmoUpdate` (`.CustomInteger` (break `InventoryItem` (`self.Inventory Item`))) (`self.AmmoMagazinSize`)))
                (`KismetSystemLibrary.Delay` (`self.FireDelay Duration`))
                (goto _label_2 :!via `Reset`))))))
      (else
        (`GameplayMessageSubsystem.K2_BroadcastMessage` (subsystem `GameplayMessageSubsystem`) (struct :`TagName` "GameplayMessage.NotEnoughAmmo") (make `EmptyPayload`))
        (`GameplayStatics.PlaySoundAtLocation` (`self.EmptyMagSound`) (`SceneComponent.K2_GetComponentLocation` (`self.SkeletalMesh`)) (struct) 1.0 1.0 0.0 null null null null)))))

(fn `UserConstructionScript`
  (`parent.UserConstructionScript`))