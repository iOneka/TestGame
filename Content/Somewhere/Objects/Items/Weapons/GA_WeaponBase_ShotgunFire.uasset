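; Gameplay ability that fires one shotgun shot from the weapon the survival character currently holds.
; On activation it caches the character, player controller and held BP_WeaponBase from the inventory component.
; It calls the weapon's multi-shell damage and recoil functions using that weapon's own stats.
; It then decrements the item's CustomInteger, clamped at zero, writes it back to the main container cell and ends.
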(event `self.K2_ActivateAbility`
  (bind _as_bp_rifle_base (`self.As BP Rifle Base`))
  (bind _as_bp_rifle_base_2 (`self.As BP Rifle Base`))
  (bind (_inventory_item_id _inventory_item_amount _inventory_item_cell _inventory_item_custominteger _inventory_item_durability _inventory_item_additionaldata) (break `InventoryItem` (`/Game/Somewhere/Core/Holdable/BP_Holdable.Inventory Item` (`self.As BP Rifle Base`))))
  (`|ExecutionSequence`
    (:`then_0`
      ;[0 0 0] Рефы
      (bind _ascharacter (cast `Character` (`self.GetAvatarActorFromActorInfo`)))
      (bind _output_get (set `self.Character` _ascharacter))
      (bind _asplayer_controller (cast `PlayerController` (`Pawn.GetController` _output_get)))
      (set `self.Player Controller` _asplayer_controller)
      (bind _asch_survival_character (cast `/Game/Somewhere/Core/Player/CH_SurvivalCharacter` (`self.Character`)))
      (set `self.As CH Survival Character` _asch_survival_character)
      (bind _asbp_weapon_base (cast `/Game/Somewhere/Objects/Items/Weapons/BP_WeaponBase` (`/Game/Somewhere/Core/Player/Inventory/BPC_InventoryComponent.Current Holdable` (`/Game/Somewhere/Core/Player/CH_SurvivalCharacter.BPC_InventoryComponent` (`self.As CH Survival Character`)))))
      (set `self.As BP Rifle Base` _asbp_weapon_base))
    (:`then_2`
      (`/Game/Somewhere/Core/Holdable/BP_Gun.Apply Damage Shotguns` _as_bp_rifle_base (`/Game/Somewhere/Objects/Items/Weapons/BP_WeaponBase.Distance` _as_bp_rifle_base) (`/Game/Somewhere/Objects/Items/Weapons/BP_WeaponBase.ShellAmount` _as_bp_rifle_base) (`/Game/Somewhere/Objects/Items/Weapons/BP_WeaponBase.Damage` _as_bp_rifle_base) (`/Game/Somewhere/Objects/Items/Weapons/BP_WeaponBase.Spread Aim` _as_bp_rifle_base) (`/Game/Somewhere/Objects/Items/Weapons/BP_WeaponBase.Spread Without Aim` _as_bp_rifle_base))
      (`/Game/Somewhere/Core/Holdable/BP_Gun.Recoil` _as_bp_rifle_base_2 (`/Game/Somewhere/Objects/Items/Weapons/BP_WeaponBase.Recoil Amp Def` _as_bp_rifle_base_2) (`/Game/Somewhere/Objects/Items/Weapons/BP_WeaponBase.Sideways Def` _as_bp_rifle_base_2) (`/Game/Somewhere/Objects/Items/Weapons/BP_WeaponBase.Min Random` _as_bp_rifle_base_2) (`/Game/Somewhere/Objects/Items/Weapons/BP_WeaponBase.Max Random` _as_bp_rifle_base_2) (`/Game/Somewhere/Objects/Items/Weapons/BP_WeaponBase.Base Look Up Rate` _as_bp_rifle_base_2) (`/Game/Somewhere/Objects/Items/Weapons/BP_WeaponBase.Base Turn Rate` _as_bp_rifle_base_2))
      (bind _output_get_2 (set `/Game/Somewhere/Core/Holdable/BP_Holdable.Inventory Item` (make `InventoryItem` _inventory_item_id _inventory_item_amount _inventory_item_cell (`KismetMathLibrary.Clamp` (- _inventory_item_custominteger 1) 0 99999) _inventory_item_durability _inventory_item_additionaldata) (`self.As BP Rifle Base`)))
      (`ItemContainer.SetCell` (`/Game/Somewhere/Core/Player/Inventory/BPC_InventoryComponent.Main Container` (`/Game/Somewhere/Core/Player/CH_SurvivalCharacter.BPC_InventoryComponent` (`self.As CH Survival Character`))) (`/Game/Somewhere/Core/Holdable/BP_Holdable.Cell Item` (`self.As BP Rifle Base`)) _output_get_2)
      (`self.K2_EndAbility`))))